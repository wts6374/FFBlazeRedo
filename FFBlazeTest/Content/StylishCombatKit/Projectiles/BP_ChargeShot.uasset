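; BP_ChargeShot is a charge-shot projectile in the Stylish Combat Kit that relies on its parent class for initialization.
; Each tick it calls the parent, then drops Speed to a low value once it has hit at least one character.
; An unconnected chain, which never runs, would attach a launching BP_Hitbox and redirect velocity and pitch toward the owner's lock-on target.
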(event EventBeginPlay
  (|CallParentFunction) ; This node is disabled and will not be called.\nDrag off pins to build functionality.
)

(event Collision|EventActorBeginOverlap
  (params (OtherActor :type Actor%20Object%20Reference)))

(event EventTick
  (params (DeltaSeconds :type Float%20%28single-precision%29))
  (|CallParentFunction DeltaSeconds)
  (if (>= (Utilities|Array|Length (Variables|Default|GetHitCharacters)) 1)
    (Variables|Default|SetSpeed 5.0)))

(event EventInitialize
  ;[1 1 1] Initialize
  (|CallParentFunction))

(fn ConstructionScript
  (|CallParentFunction))