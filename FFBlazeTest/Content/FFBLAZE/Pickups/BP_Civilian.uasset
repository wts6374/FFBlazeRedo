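; BP_Civilian is an interactable civilian that the player rescues for a fixed money reward.
; Interact casts to BP_BaseCharacter, pays through ManageMoney, disables the box collision and plays the Rescue animation.
; After a delay it plays a coin sound at world origin, spawns a teleport effect, and clears the Interaction flag.
; Colected then hides the civilian, light and text without destroying the actor.
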(event Custom|Colected
  (Rendering|SetVisibility (Variables|Default|GetCivilian) false false)
  (Collision|SetCollisionEnabled (Variables|Default|GetBox) "NoCollision")
  (Rendering|SetVisibility (Variables|Default|GetPointLight) false false)
  (Rendering|SetVisibility (Variables|Default|GetTextRender) false false))

(event EventBeginPlay
  (Variables|Default|SetInteraction true))

(event EventInteract
  (params (Player :type Character%20Object%20Reference))
  (Utilities|IsValid Player
    (:Is%20Valid
      (bind _asbp_base_character (Utilities|Casting|CastToBP_BaseCharacter Player))
      (Variables|Default|SetNewPlayer _asbp_base_character)
      (if (and (Utilities|IsValid (Variables|Default|GetNewPlayer)) (Variables|Default|GetInteraction))
        (Default|ManageMoney (Variables|Default|GetNewPlayer) 1000)
        (Collision|SetCollisionEnabled (Variables|Default|GetBox) "NoCollision")
        (Components|Animation|PlayAnimation (Variables|Default|GetCivilian) "/Game/FFBLAZE/Pickups/Rescue.Rescue" false)
        (Utilities|FlowControl|Delay 2.75)
        (Audio|PlaySoundatLocation "/Game/FFBLAZE/Sound/ShopOrCurrencySFX/collected_coin_sound.collected_coin_sound" "0, 0, 0" "0, 0, 0" 1.0 1.0 0.0 0 0 0)
        (Effects|SpawnEmitteratLocation "/Game/StylishCombatKit/VFX/ParticleSystems/P_TeleportBlue.P_TeleportBlue" (Transformation|GetActorLocation) "0, 0, 0" "1.000000,1.000000,1.000000" false)
        (Rendering|SetVisibility (Variables|Default|GetCivilian) false false)
        (Collision|SetCollisionEnabled (Variables|Default|GetBox) "NoCollision")
        (Variables|Default|SetInteraction false)
        (CallFunction|Colected)))))

(fn ConstructionScript)