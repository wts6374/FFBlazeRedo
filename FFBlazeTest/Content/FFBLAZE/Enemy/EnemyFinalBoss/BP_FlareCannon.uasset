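; BP_FlareCannon is a final boss attack actor, built on a character-style parent, that creates a long beam-shaped damage zone.
; On Initialize it spawns sixteen BP_Hitbox actors it owns, attaches them to its capsule and spaces them evenly along its forward axis as large overlapping spheres.
; Each hitbox gets the same damage and launch HitData and activates immediately, then the cannon zeroes its movement velocity.
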(event EventBeginPlay
  (|CallParentFunction) ; This node is disabled and will not be called.\nDrag off pins to build functionality.
)

(event Collision|EventActorBeginOverlap
  (params (OtherActor :type Actor%20Object%20Reference)))

(event EventTick
  (params (DeltaSeconds :type Float%20%28single-precision%29))
  (|CallParentFunction DeltaSeconds) ; This node is disabled and will not be called.\nDrag off pins to build functionality.
)

(event EventInitialize
  ;[1 1 1] Initialize
  (|CallParentFunction)
  (for _index (range 0 15)
    (bind _returnvalue (Game|SpawnActorfromClass "/Game/StylishCombatKit/Misc/BP_Hitbox.BP_Hitbox_C" (Transformation|GetActorTransform) "AlwaysSpawn" 0 0))
    (Variables|/Game/StylishCombatKit/Misc/BP_Hitbox.BP_Hitbox_C|SetOwnerCharacter _returnvalue self)
    (Transformation|AttachComponentToComponent _returnvalue (Variables|Default|GetCapsuleComponent) "None" "KeepWorld" "KeepWorld" "KeepWorld" true)
    (Transformation|SetActorRelativeLocation _returnvalue (Utilities|Select :Index _index :Option%200 "200.000000,0.000000,30.000000" :Option%201 "400.000000,0.000000,30.000000" :Option%202 "600.000000,0.000000,30.000000" :Option%203 "800.000000, 0,30.000000" :Option%204 "1000.000000, 0,30.000000" :Option%205 "1200.000000, 0,30.000000" :Option%206 "1400.000000,0.000000,30.000000" :Option%207 "1600.000000, 0,30.000000" :Option%208 "1800.000000, 0,30.000000" :Option%209 "2000.000000, 0,30.000000" :Option%2010 "2200.000000, 0,30.000000" :Option%2011 "2400.000000, 0,30.000000" :Option%2012 "2600.000000, 0,30.000000" :Option%2013 "2800.000000, 0,30.000000" :Option%2014 "3000.000000, 0,30.000000" :Option%2015 "3200.000000, 0,30.000000"))
    (Utilities|Array|Add (Variables|Default|GetHitboxes) _returnvalue)
    (Components|Sphere|SetSphereRadius (Variables|/Game/StylishCombatKit/Misc/BP_Hitbox.BP_Hitbox_C|GetHitbox _returnvalue) 2.5e+02 true)
    (Variables|/Game/StylishCombatKit/Misc/BP_Hitbox.BP_Hitbox_C|SetHitData _returnvalue (Utilities|Struct|MakeStruct_HitData 1 "-100.000000,0.000000,50.000000" 5.0 2 0.05 0.5 0.0 false))
    (Default|Activate _returnvalue true))
  (bind _output_get (Variables|/Script/Engine.MovementComponent|SetVelocity (Variables|Character|GetCharacterMovement) "0, 0, 0"))
  (Variables|Default|SetPreviousFrameVelocity _output_get))

(fn ConstructionScript
  (|CallParentFunction))