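; BP_Gun is a gun-wielding Hothead enemy that locks onto the player and shows a health widget.
; Light attacks turn the AI action index into simulated directional input, choosing gun montages for flips, charges and teleport-effect backflips.
; Water drains cascading temperature tiers that drive materials and TriggerActive, disabling attacks at zero until a timed refill.
; It also handles hurt, landing and death, which drops MoneywaterRefill pickups, and socket-attaches its hurtboxes.
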(event Custom|ChangeLook
  (bind _mesh (Variables|Character|GetMesh))
  (bind _mesh_2 (Variables|Character|GetMesh))
  (bind _mesh_3 (Variables|Character|GetMesh))
  (bind _mesh_4 (Variables|Character|GetMesh))
  (bind _mesh_5 (Variables|Character|GetMesh))
  ;[1 1 1] Attack command
  ;;[1 1 1] Change material based on Temperature
  (switch int (Variables|Default|GetTempTier)
    (:0
      (Rendering|Material|SetMaterial _mesh_4 0 "/Game/FFBLAZE/Enemy/EnemyColors/Cool.Cool")
      (Rendering|Material|SetMaterial _mesh_4 1 "/Game/FFBLAZE/Enemy/EnemyColors/CoolOutline.CoolOutline"))
    (:1
      (Rendering|Material|SetMaterial _mesh 1 "/Game/FFBLAZE/Enemy/EnemyColors/WarmOutline.WarmOutline")
      (Rendering|Material|SetMaterial _mesh 0 "/Game/FFBLAZE/Enemy/EnemyColors/Warm.Warm"))
    (:2
      (Rendering|Material|SetMaterial _mesh_5 0 "/Game/FFBLAZE/Enemy/EnemyColors/Hottie.Hottie")
      (Rendering|Material|SetMaterial _mesh_5 1 "/Game/FFBLAZE/Enemy/EnemyColors/WarmOutline.WarmOutline"))
    (:3
      (Rendering|Material|SetMaterial _mesh_2 0 "/Game/FFBLAZE/Enemy/EnemyColors/RedHot.RedHot")
      (Rendering|Material|SetMaterial _mesh_2 1 "/Game/FFBLAZE/Enemy/EnemyColors/RedHotOutline.RedHotOutline"))
    (:4
      (Rendering|Material|SetMaterial _mesh_3 0 "/Game/FFBLAZE/Enemy/EnemyColors/WhiteHot.WhiteHot")
      (Rendering|Material|SetMaterial _mesh_3 1 "/Game/FFBLAZE/Enemy/EnemyColors/WhitHotOutline.WhitHotOutline"))))

(event Custom|ChargeTimer
  ;[1 1 1] Attack command
  ;;[1 1 1] Input attack button and hold for specified charge time
  (bind _output_get (Variables|Default|SetLightButton false))
  (|CallParentFunction _output_get)
  (bind _output_get_2 (Variables|Default|SetHeavyButton false))
  (CallFunction|InputHeavyAttack _output_get_2))

(event Custom|UpdateUI
  (bind _healthwidget (Variables|Default|GetHealthWidget))
  ;[1 1 1] Update UI
  (Variables|/Game/FFBLAZE/UI/EnemyHealth.EnemyHealth_C|SetEnemy (Variables|Default|GetUIBar) self)
  (if (Variables|Default|GetIsLockedOn)
    (Rendering|SetVisibility _healthwidget true false)
    (else
      (Rendering|SetVisibility _healthwidget false false))))

(event Custom|StartUI
  ;[1 1 1] Update UI
  (bind _asenemy_health (Utilities|Casting|CastToEnemyHealth (UserInterface|GetUserWidgetObject (Variables|Default|GetHealthWidget))))
  (Variables|Default|SetUIBar _asenemy_health))

(event EventBeginPlay
  ;[1 1 1] Initialize
  (|CallParentFunction)
  (bind _asbp_base_character (Utilities|Casting|CastToBP_BaseCharacter (Game|GetPlayerCharacter 0)))
  (Variables|Default|SetLockOnTarget _asbp_base_character)
  (Variables|Default|SetIsLockedOn true)
  (Variables|Default|SetLockonButton true)
  (CallFunction|StartUI))

(event EventCollisionStopTriggered
  ;[1 1 1] Dash Punch Collision Trigger
)

(event EventFlinch
  ;[1 1 1] Hurt animation
  (Animation|PlayAnimMontage (select (Variables|Default|GetInAir) "/Game/FFBLAZE/Enemy/EnemyHotheads/HH_AirHit.HH_AirHit" "/Game/FFBLAZE/Enemy/EnemyHotheads/HH_hit.HH_hit") 1.0 ""))

(event EventNeutralDirectionHoldButtonInput
  ;[1 1 1] Dash Punch Collision Trigger
)

(event EventAdjustTemperature
  (params (WaterIntake :type Float%20%28single-precision%29))
  ;[1 1 1] Change target temperature
  (if (== (Variables|Default|GetTempTier) 4)
    (bind _output_get (Variables|Default|SetWhiteHottemp (- (Variables|Default|GetWhiteHottemp) WaterIntake)))
    (if (<= _output_get 0.0)
      (Variables|Default|SetTempTier 3)
      (if (< (- (Variables|Default|GetWhiteHottemp) WaterIntake) 0.0)
        (CallFunction|AdjustTemperature (* (- (Variables|Default|GetWhiteHottemp) WaterIntake) -1.0))))
    (elif (== (Variables|Default|GetTempTier) 3)
      (bind _output_get_2 (Variables|Default|SetRedHotTemp (- (Variables|Default|GetRedHotTemp) WaterIntake)))
      (if (<= _output_get_2 0.0)
        (Variables|Default|SetTempTier 2)
        (if (< (- (Variables|Default|GetRedHotTemp) WaterIntake) 0.0)
          (CallFunction|AdjustTemperature (* (- (Variables|Default|GetRedHotTemp) WaterIntake) -1.0))))
      (elif (== (Variables|Default|GetTempTier) 2)
        (bind _output_get_3 (Variables|Default|SetHotTemp (- (Variables|Default|GetHotTemp) WaterIntake)))
        (if (<= _output_get_3 0.0)
          (Variables|Default|SetTempTier 1)
          (if (< (- (Variables|Default|GetHotTemp) WaterIntake) 0.0)
            (CallFunction|AdjustTemperature (* (- (Variables|Default|GetHotTemp) WaterIntake) -1.0))))
        (elif (== (Variables|Default|GetTempTier) 1)
          (bind _output_get_4 (Variables|Default|SetMidTemp (- (Variables|Default|GetMidTemp) WaterIntake)))
          (if (<= _output_get_4 0.0)
            (Variables|Default|SetTempTier 0)
            (if (< (- (Variables|Default|GetMidTemp) WaterIntake) 0.0)
              (CallFunction|AdjustTemperature (* (- (Variables|Default|GetMidTemp) WaterIntake) -1.0))))
          (else
            (Variables|Default|SetTempTier 0)
            (Variables|Default|SetStartRefll true)
            (Variables|Default|SetRefillTimer (Math|Float|Clamp(Float) (+ (Variables|Default|GetRefillTimer) (* WaterIntake 0.0)) 0.0 (Variables|Default|GetRefillTimerMax)))))))))

(event EventForceLand
  ;[1 1 1] Land
  (Variables|Default|SetInAir false)
  (if (and (== (Variables|Default|GetStateIndex) 2) (== (Variables|Default|GetSubStateIndex) 4))
    (Animation|PlayAnimMontage "/Game/FFBLAZE/Enemy/EnemyHotheads/GunFlip.GunFlip" 1.0 "Land")
    (CallFunction|ResetAirOptions :!label _label)
    (CallFunction|RestoreMovementDefaults false)
    (Variables|Default|SetCombatAnimation true)
    (elif (== (Variables|Default|GetStateIndex) 4)
      (Animation|PlayAnimMontage "/Game/FFBLAZE/Enemy/EnemyHotheads/HH_knockdown.HH_knockdown" 1.0 "")
      (goto _label)
      (elif (== (Variables|Default|GetStateIndex) 5)
        (Animation|PlayAnimMontage "/Game/FFBLAZE/Enemy/EnemyHotheads/HH_Dead.HH_Dead" 1.0 "Explode")
        (else
          (Animation|PlayAnimMontage "/Game/FFBLAZE/Enemy/EnemyHotheads/HHLand_Montage.HHLand_Montage" 1.0 "")
          (CallFunction|CanDo true true)
          (CallFunction|ResetAirOptions)
          (CallFunction|StartAnim)
          (CallFunction|RestoreMovementDefaults false)
          (Variables|Default|SetCombatAnimation false)
          (CallFunction|ReleaseBuffer))))))

(event EventInputLightAttack
  (params (Pressed :type Boolean))
  (bind _rotation (CallFunction|CameraYaw))
  (bind _returnvalue (Transformation|GetActorLocation))
  (bind _aicontrollerref (Variables|Default|GetAIControllerRef))
  (bind _lockontarget (Variables|Default|GetLockOnTarget))
  (bind _charactermovement (Variables|Character|GetCharacterMovement))
  (bind _charactermovement_2 (Variables|Character|GetCharacterMovement))
  (bind _returnvalue_2 (Transformation|GetActorLocation _lockontarget))
  (bind _aiactionindex (Variables|/Game/StylishCombatKit/AI/AIC_Enemy.AIC_Enemy_C|GetAIActionIndex _aicontrollerref))
  (bind _returnvalue_3 (Math|Vector|GetUnitDirection(Vector) _returnvalue _returnvalue_2))
  (bind (_x _y) (Math|Vector|BreakVector _returnvalue_3))
  (bind _returnvalue_4 (Math|Vector|MakeVector _x _y 0.0))
  (bind _returnvalue_5 (Math|Vector|Normalize _returnvalue_4))
  (bind _returnvalue_6 (Math|Vector|UnrotateVector _returnvalue_5 _rotation))
  (bind _returnvalue_7 (Math|Conversions|ToVector2D(Vector) _returnvalue_6))
  (bind (_x_2 _y_2) (Math|Vector2D|BreakVector2D _returnvalue_7))
  (bind _returnvalue_8 (Math|Vector2D|MakeVector2D _y_2 _x_2))
  (bind _returnvalue_9 (* _returnvalue_8 -1.0))
  (bind _returnvalue_10 (Utilities|Select :Index _aiactionindex :Option%200 _returnvalue_9 :Option%201 "" :Option%202 _returnvalue_8 :Option%203 ""))
  ;[1 1 1] Attack command
  (if (and (Variables|Default|GetCanAttack) (> (Variables|Default|GetTempTier) 0))
    (if (Variables|Default|GetInAir)
      (if (or (< (Variables|Default|GetAirJumpsUsed) 2) (not (Variables|Default|GetInAir)))
        (Variables|Default|SetInputVector _returnvalue_10)
        (Variables|Default|SetAirJumpsUsed (- (Variables|Default|GetAirJumpsUsed) -1))
        (switch int (+ (select (== (Variables|Default|GetInputBuffer) 3) (Variables|Default|GetDirectionBuffer) (CallFunction|DirectionalInput)) 1)
          (:Default
            (CallFunction|OrientCharacter true true :!label _label)
            (CallFunction|CanDo false true)
            (CallFunction|StartAnim)
            (Animation|PlayAnimMontage "/Game/FFBLAZE/Enemy/EnemyHotheads/GunFlipback.GunFlipback" 1.0 "")
            (Variables|Default|SetStateIndex 2)
            (Variables|Default|SetSubStateIndex 5))
          (:0
            (goto _label))
          (:1
            (CallFunction|OrientCharacter true true)
            (CallFunction|CanDo false true)
            (CallFunction|StartAnim)
            (Animation|PlayAnimMontage "/Game/FFBLAZE/Enemy/EnemyHotheads/GunFlip.GunFlip" 1.0 "")
            (Variables|Default|SetStateIndex 2)
            (Variables|Default|SetSubStateIndex 4)))
        (Variables|/Script/Engine.CharacterMovementComponent|SetGravityScale _charactermovement_2 5.0)
        (Variables|/Script/Engine.MovementComponent|SetVelocity _charactermovement_2 (+ (* (Variables|/Script/Engine.MovementComponent|GetVelocity _charactermovement_2) "0.500000,0.500000,0.000000") "0, 0,700.000000"))
        (Variables|Default|SetFloatTime 0.2)
        (CallFunction|UpdateRecentMoves -1))
      (else
        ;;[1 1 1] Set input vector to simulate directional inputs
        (Variables|Default|SetInputVector _returnvalue_10)
        ;;[1 1 1] Input attack button and hold for specified charge time
        (if (== _aiactionindex 3)
          (if (or (< (Variables|Default|GetAirTeleportsUsed) 1) (not (Variables|Default|GetInAir)))
            (Variables|/Script/Engine.MovementComponent|SetVelocity _charactermovement (+ (* (Transformation|GetActorForwardVector) 5e+01) "0, 0,100.000000"))
            (Variables|Default|SetFloatTime 0.2)
            (Variables|/Script/Engine.CharacterMovementComponent|SetGravityScale _charactermovement 2.0)
            (CallFunction|StartAnim)
            (CallFunction|CanDo false true)
            (CallFunction|OrientCharacter true true)
            (Animation|PlayAnimMontage "/Game/FFBLAZE/Enemy/EnemyHotheads/GunFlipback.GunFlipback" 1.0 "")
            (Variables|Default|SetStateIndex 2)
            (Variables|Default|SetSubStateIndex 5)
            (if (Variables|Default|GetInAir)
              (Math|Integer|IncrementInt (Variables|Default|GetAirTeleportsUsed)
                (:%20%20
                  _)))
            (Variables|Default|SetInputBuffer 0)
            (CallFunction|CanDo false true)
            (Effects|SpawnEmitteratLocation "/Game/StylishCombatKit/VFX/ParticleSystems/P_TeleportRed.P_TeleportRed" (Transformation|GetActorLocation))
            (CallFunction|UpdateRecentMoves -1 :!label _label_2)
            (Utilities|Time|SetTimerbyEvent (delegate Custom|ChargeTimer) 0.3))
          (else
            (CallFunction|StartAnim)
            (CallFunction|CanDo false true)
            (CallFunction|OrientCharacter true true)
            (switch int (+ (select (== (Variables|Default|GetInputBuffer) 3) (Variables|Default|GetDirectionBuffer) (CallFunction|DirectionalInput)) 1)
              (:Default
                _)
              (:0
                (Animation|PlayAnimMontage "/Game/FFBLAZE/Enemy/EnemyHotheads/GunFlip.GunFlip" 1.0 "")
                (Variables|Default|SetStateIndex 2)
                (Variables|Default|SetSubStateIndex 4)
                (goto _label_2))
              (:1
                (Animation|PlayAnimMontage "/Game/FFBLAZE/Enemy/EnemyHotheads/GunCharge.GunCharge" 1.0 "")
                (Variables|Default|SetStateIndex 2)
                (Variables|Default|SetSubStateIndex 3)
                (goto _label_2))
              (:2
                _))
            (Animation|PlayAnimMontage "/Game/FFBLAZE/Enemy/EnemyHotheads/GunAttack.GunAttack" 1.0 "")
            (Variables|Default|SetStateIndex 2)
            (Variables|Default|SetSubStateIndex 5)
            (goto _label_2)))))))

(event EventOnLanded
  (params (Hit :type Hit%20Result%20Structure%20%28by%20ref%29))
  ;[1 1 1] Land
  (Variables|Default|SetInAir false)
  (if (and (== (Variables|Default|GetStateIndex) 2) (== (Variables|Default|GetSubStateIndex) 4))
    (Animation|PlayAnimMontage "/Game/FFBLAZE/Enemy/EnemyHotheads/GunFlip.GunFlip" 1.0 "Land")
    (CallFunction|ResetAirOptions :!label _label)
    (CallFunction|RestoreMovementDefaults false)
    (Variables|Default|SetCombatAnimation true)
    (elif (== (Variables|Default|GetStateIndex) 4)
      (Animation|PlayAnimMontage "/Game/FFBLAZE/Enemy/EnemyHotheads/HH_knockdown.HH_knockdown" 1.0 "")
      (goto _label)
      (elif (== (Variables|Default|GetStateIndex) 5)
        (Animation|PlayAnimMontage "/Game/FFBLAZE/Enemy/EnemyHotheads/HH_Dead.HH_Dead" 1.0 "Explode")
        (else
          (Animation|PlayAnimMontage "/Game/FFBLAZE/Enemy/EnemyHotheads/HHLand_Montage.HHLand_Montage" 1.0 "")
          (CallFunction|CanDo true true)
          (CallFunction|ResetAirOptions)
          (CallFunction|StartAnim)
          (CallFunction|RestoreMovementDefaults false)
          (Variables|Default|SetCombatAnimation false)
          (CallFunction|ReleaseBuffer))))))

(event EventHurtAnimation
  (params (AttackerHitbox :type BP%20Hitbox%20Object%20Reference))
  ;[1 1 1] Hurt animation
  (if (Variables|Default|GetInAir)
    (Animation|PlayAnimMontage "/Game/FFBLAZE/Enemy/EnemyHotheads/HH_AirHit.HH_AirHit" 1.0 "")
    (else
      (Animation|PlayAnimMontage "/Game/FFBLAZE/Enemy/EnemyHotheads/HH_hit.HH_hit" 1.0 "")))
  (CallFunction|StartAnim)
  (CallFunction|CanDo false true)
  (Variables|Default|SetCanEnemyStep false)
  (Variables|Default|SetStateIndex 4))

(event EventDeathAnimation
  ;[1 1 1] Hurt animation
  (Animation|PlayAnimMontage "/Game/FFBLAZE/Enemy/EnemyHotheads/HH_Dead.HH_Dead" 1.0 "")
  (Variables|Default|SetTargetGravity 0.0)
  (Variables|Default|SetFloatTime 3.0)
  (for _index (range 0 5)
    (Game|SpawnActorfromClass "/Game/FFBLAZE/Pickups/MoneywaterRefill.MoneywaterRefill_C" (Transformation|GetActorTransform) "Undefined" 0 0))
  (Utilities|FlowControl|Delay 1.3)
  (Actor|DestroyActor))

(event EventTick
  (params (DeltaSeconds :type Float%20%28single-precision%29))
  ;[1 1 1] Updater
  (|CallParentFunction DeltaSeconds)
  (CallFunction|ChangeLook)
  (CallFunction|UpdateUI)
  (if (>= (Variables|Default|GetTempTier) 2)
    (Variables|Default|SetTriggerActive true)
    (else
      (Variables|Default|SetTriggerActive false))))

(event EventRegainTemp
  ;[1 1 1] Regains Temperature if depleted
  (if (Variables|Default|GetStartRefll)
    (if (> (Variables|Default|GetRefillTimer) 0.0)
      (Variables|Default|SetRefillTimer (- (Variables|Default|GetRefillTimer) (* (Utilities|Time|GetWorldDeltaSeconds) 2.0)))
      (else
        (Variables|Default|SetRefillTimer (Variables|Default|GetRefillTimerMax))
        (Variables|Default|SetStartRefll false)
        (Variables|Default|SetWhiteHottemp (Variables|Default|GetWhiteHottempMax))
        (Variables|Default|SetRedHotTemp (Variables|Default|GetRedHotTempMax))
        (Variables|Default|SetHotTemp (Variables|Default|GetHotTempMax))
        (Variables|Default|SetMidTemp (Variables|Default|GetMidTempMax))
        (Variables|Default|SetTempTier (Variables|Default|GetTempTierMax))
        (CallFunction|StartAnim)
        (CallFunction|CanDo false true)
        (CallFunction|OrientCharacter true true)
        (Animation|PlayAnimMontage "/Game/FFBLAZE/Enemy/EnemyHotheads/HH_hit.HH_hit" 1.0 "")
        (Variables|Default|SetStateIndex 2)
        (Variables|Default|SetSubStateIndex 5)))))

(fn ConstructionScript
  (bind _mesh (Variables|Character|GetMesh))
  (|CallParentFunction)
  (Transformation|AttachComponentToComponent (Variables|Default|GetHurtboxTorso) _mesh "spine_03" "KeepRelative" "KeepRelative" "KeepRelative" true)
  (Transformation|AttachComponentToComponent (Variables|Default|GetHurtboxLegL) _mesh "calf_l" "KeepRelative" "KeepRelative" "KeepRelative" true)
  (Transformation|AttachComponentToComponent (Variables|Default|GetHurtboxLegR) _mesh "calf_r" "KeepRelative" "KeepRelative" "KeepRelative" true)
  (Transformation|AttachComponentToComponent (Variables|Default|GetRepelSphere) _mesh "spine_03" "KeepRelative" "KeepRelative" "KeepRelative" true)
  (Variables|Default|SetHurtboxes (Utilities|Array|MakeArray (Variables|Default|GetHurtboxTorso) (Variables|Default|GetHurtboxLegL) (Variables|Default|GetHurtboxLegR))))