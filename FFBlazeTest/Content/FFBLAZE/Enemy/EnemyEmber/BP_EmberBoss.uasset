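; Ember boss enemy that locks onto the player and fights through temperature tiers cooled by water.
; AI action index drives fire breath or simulated camera-relative directional input selecting bite, dive or charge montages, with a timer releasing the attack buttons.
; Water intake drains each tier, passing excess down; tiers swap materials and gate attacks, which stop at tier zero.
; Also handles hurt and landing animations, health widget, socketed hurtboxes, and water-refill drops on death.
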(event Custom|ChargeTimer
  ;[1 1 1] Attack command
  ;;[1 1 1] Input attack button and hold for specified charge time
  (bind _output_get (Variables|Default|SetLightButton false))
  (|CallParentFunction _output_get)
  (bind _output_get_2 (Variables|Default|SetHeavyButton false))
  (CallFunction|InputHeavyAttack _output_get_2))

(event Custom|ChangeLook
  (bind _mesh (Variables|Character|GetMesh))
  (bind _mesh_2 (Variables|Character|GetMesh))
  (bind _mesh_3 (Variables|Character|GetMesh))
  (bind _mesh_4 (Variables|Character|GetMesh))
  (bind _mesh_5 (Variables|Character|GetMesh))
  ;[1 1 1] Attack command
  ;;[1 1 1] Change material based on Temperature
  (switch int (Variables|Default|GetTempTier)
    (:0
      (Rendering|Material|SetMaterial _mesh_5 0 "/Game/FFBLAZE/Enemy/EnemyColors/Cool.Cool")
      (Rendering|Material|SetMaterial _mesh_5 1 "/Game/FFBLAZE/Enemy/EnemyColors/CoolOutline.CoolOutline"))
    (:1
      (Rendering|Material|SetMaterial _mesh_3 1 "/Game/FFBLAZE/Enemy/EnemyColors/WarmOutline.WarmOutline")
      (Rendering|Material|SetMaterial _mesh_3 0 "/Game/FFBLAZE/Enemy/EnemyColors/Warm.Warm"))
    (:2
      (Rendering|Material|SetMaterial _mesh_2 0 "/Game/FFBLAZE/Enemy/EnemyColors/Hottie.Hottie")
      (Rendering|Material|SetMaterial _mesh_2 1 "/Game/FFBLAZE/Enemy/EnemyColors/WarmOutline.WarmOutline"))
    (:3
      (Rendering|Material|SetMaterial _mesh 0 "/Game/FFBLAZE/Enemy/EnemyColors/RedHot.RedHot")
      (Rendering|Material|SetMaterial _mesh 1 "/Game/FFBLAZE/Enemy/EnemyColors/RedHotOutline.RedHotOutline"))
    (:4
      (Rendering|Material|SetMaterial _mesh_4 0 "/Game/FFBLAZE/Enemy/EnemyColors/WhiteHot.WhiteHot")
      (Rendering|Material|SetMaterial _mesh_4 1 "/Game/FFBLAZE/Enemy/EnemyColors/WhitHotOutline.WhitHotOutline"))))

(event Custom|CustomEvent
  (params (WaterIntake :type Float%20%28single-precision%29))
  ;[1 1 1] Change target temperature
  (if (== (Variables|Default|GetTempTier) 4)
    (bind _output_get (Variables|Default|SetWhiteHottemp (- (Variables|Default|GetWhiteHottemp) WaterIntake)))
    (if (<= _output_get 0.0)
      (Variables|Default|SetTempTier 3)
      (if (< (- (Variables|Default|GetWhiteHottemp) WaterIntake) 0.0)
        (CallFunction|AdjustTemperature (* (- (Variables|Default|GetWhiteHottemp) WaterIntake) -1.0))))
    (elif (== (Variables|Default|GetTempTier) 3)
      (bind _output_get_2 (Variables|Default|SetRedHotTemp (- (Variables|Default|GetRedHotTemp) WaterIntake)))
      (if (<= _output_get_2 0.0)
        (Variables|Default|SetTempTier 2)
        (if (< (- (Variables|Default|GetRedHotTemp) WaterIntake) 0.0)
          (CallFunction|AdjustTemperature (* (- (Variables|Default|GetRedHotTemp) WaterIntake) -1.0))))
      (elif (== (Variables|Default|GetTempTier) 2)
        (bind _output_get_3 (Variables|Default|SetHotTemp (- (Variables|Default|GetHotTemp) WaterIntake)))
        (if (<= _output_get_3 0.0)
          (Variables|Default|SetTempTier 1)
          (if (< (- (Variables|Default|GetHotTemp) WaterIntake) 0.0)
            (CallFunction|AdjustTemperature (* (- (Variables|Default|GetHotTemp) WaterIntake) -1.0))))
        (elif (== (Variables|Default|GetTempTier) 1)
          (bind _output_get_4 (Variables|Default|SetMidTemp (- (Variables|Default|GetMidTemp) WaterIntake)))
          (if (<= _output_get_4 0.0)
            (Variables|Default|SetTempTier 0)
            (if (< (- (Variables|Default|GetMidTemp) WaterIntake) 0.0)
              (CallFunction|AdjustTemperature (* (- (Variables|Default|GetMidTemp) WaterIntake) -1.0))))
          (else
            (Variables|Default|SetTempTier 0)
            (Variables|Default|SetStartRefll true)))))))

(event Custom|UpdateUI
  (bind _healthwidget (Variables|Default|GetHealthWidget))
  ;[1 1 1] Update UI
  (Variables|/Game/FFBLAZE/UI/EnemyHealth.EnemyHealth_C|SetEnemy (Variables|Default|GetUIBar) self)
  (if (Variables|Default|GetIsLockedOn)
    (Rendering|SetVisibility _healthwidget true false)
    (else
      (Rendering|SetVisibility _healthwidget false false))))

(event Custom|StartUI
  ;[1 1 1] Update UI
  (bind _asenemy_health (Utilities|Casting|CastToEnemyHealth (UserInterface|GetUserWidgetObject (Variables|Default|GetHealthWidget))))
  (Variables|Default|SetUIBar _asenemy_health))

(event EventBeginPlay
  ;[1 1 1] Initialize
  (|CallParentFunction)
  (bind _asbp_base_character (Utilities|Casting|CastToBP_BaseCharacter (Game|GetPlayerCharacter 0)))
  (Variables|Default|SetLockOnTarget _asbp_base_character)
  (Variables|Default|SetIsLockedOn true)
  (Variables|Default|SetLockonButton true)
  (CallFunction|StartUI))

(event EventFlinch
  ;[1 1 1] Hurt animation
  (Animation|PlayAnimMontage (select (Variables|Default|GetInAir) "/Game/FFBLAZE/Enemy/EnemyEmber/EmberairHit.EmberairHit" "/Game/FFBLAZE/Enemy/EnemyEmber/EmberHit.EmberHit") 1.0 ""))

(event EventForceLand
  ;[1 1 1] Land
  (Variables|Default|SetInAir false)
  (if (and (== (Variables|Default|GetStateIndex) 2) (== (Variables|Default|GetSubStateIndex) 3))
    (Animation|PlayAnimMontage "/Game/FFBLAZE/Enemy/EnemyEmber/EmberDive.EmberDive" 1.0 "Land")
    (CallFunction|ResetAirOptions :!label _label)
    (CallFunction|RestoreMovementDefaults false)
    (Variables|Default|SetCombatAnimation true)
    (elif (== (Variables|Default|GetStateIndex) 4)
      (Animation|PlayAnimMontage "/Game/FFBLAZE/Enemy/EnemyEmber/EmberairHit.EmberairHit" 1.0 "Land")
      (goto _label)
      (elif (== (Variables|Default|GetStateIndex) 5)
        (Animation|PlayAnimMontage "/Game/FFBLAZE/Enemy/EnemyEmber/Emberdead.Emberdead" 1.0 "Explode")
        (else
          (Animation|PlayAnimMontage "/Game/FFBLAZE/Enemy/EnemyEmber/Land_Montage.Land_Montage" 1.0 "")
          (CallFunction|CanDo true true)
          (CallFunction|ResetAirOptions)
          (CallFunction|StartAnim)
          (CallFunction|RestoreMovementDefaults false)
          (Variables|Default|SetCombatAnimation false)
          (CallFunction|ReleaseBuffer))))))

(event EventInputLightAttack
  (params (Pressed :type Boolean))
  (bind _rotation (CallFunction|CameraYaw))
  (bind _returnvalue (Transformation|GetActorLocation))
  (bind _aicontrollerref (Variables|Default|GetAIControllerRef))
  (bind _lockontarget (Variables|Default|GetLockOnTarget))
  (bind _returnvalue_2 (Transformation|GetActorLocation _lockontarget))
  (bind _aiactionindex (Variables|/Game/StylishCombatKit/AI/AIC_Enemy.AIC_Enemy_C|GetAIActionIndex _aicontrollerref))
  (bind _returnvalue_3 (Math|Vector|GetUnitDirection(Vector) _returnvalue _returnvalue_2))
  (bind (_x _y) (Math|Vector|BreakVector _returnvalue_3))
  (bind _returnvalue_4 (Math|Vector|MakeVector _x _y 0.0))
  (bind _returnvalue_5 (Math|Vector|Normalize _returnvalue_4))
  (bind _returnvalue_6 (Math|Vector|UnrotateVector _returnvalue_5 _rotation))
  (bind _returnvalue_7 (Math|Conversions|ToVector2D(Vector) _returnvalue_6))
  (bind (_x_2 _y_2) (Math|Vector2D|BreakVector2D _returnvalue_7))
  (bind _returnvalue_8 (Math|Vector2D|MakeVector2D _y_2 _x_2))
  ;[1 1 1] Attack command
  (if (and (Variables|Default|GetCanAttack) (> (Variables|Default|GetTempTier) 0))
    (if (not (Variables|Default|GetInAir))
      ;;[1 1 1] Set input vector to simulate directional inputs
      (Variables|Default|SetInputVector (Utilities|Select :Index _aiactionindex :Option%200 (* _returnvalue_8 -1.0) :Option%201 "" :Option%202 _returnvalue_8 :Option%203 ""))
      ;;[1 1 1] Input attack button and hold for specified charge time
      (if (== _aiactionindex 3)
        (CallFunction|StartAnim)
        (CallFunction|CanDo false true)
        (CallFunction|OrientCharacter true true)
        (Animation|PlayAnimMontage "/Game/FFBLAZE/Enemy/EnemyEmber/EmberFire.EmberFire" 0.76 "")
        (Variables|Default|SetStateIndex 2)
        (Variables|Default|SetSubStateIndex 20)
        (else
          (CallFunction|StartAnim)
          (CallFunction|CanDo false true)
          (CallFunction|OrientCharacter true true)
          (switch int (+ (select (== (Variables|Default|GetInputBuffer) 3) (Variables|Default|GetDirectionBuffer) (CallFunction|DirectionalInput)) 1)
            (:0
              (Animation|PlayAnimMontage "/Game/FFBLAZE/Enemy/EnemyEmber/Bite.Bite" 0.7 "")
              (Variables|Default|SetStateIndex 2)
              (Variables|Default|SetSubStateIndex 5))
            (:1
              (Animation|PlayAnimMontage "/Game/FFBLAZE/Enemy/EnemyEmber/EmberDive.EmberDive" 0.5 "")
              (Variables|Default|SetStateIndex 2)
              (Variables|Default|SetSubStateIndex 3))
            (:2
              (Animation|PlayAnimMontage "/Game/FFBLAZE/Enemy/EnemyEmber/EmberCharge.EmberCharge" 0.8 "")
              (Variables|Default|SetStateIndex 2)
              (Variables|Default|SetSubStateIndex 4)))))
      (CallFunction|UpdateRecentMoves -1)
      (Utilities|Time|SetTimerbyEvent (delegate Custom|ChargeTimer) 0.3))))

(event EventOnLanded
  (params (Hit :type Hit%20Result%20Structure%20%28by%20ref%29))
  ;[1 1 1] Land
  (Variables|Default|SetInAir false)
  (if (and (== (Variables|Default|GetStateIndex) 2) (== (Variables|Default|GetSubStateIndex) 3))
    (Animation|PlayAnimMontage "/Game/FFBLAZE/Enemy/EnemyEmber/EmberDive.EmberDive" 1.0 "Land")
    (CallFunction|ResetAirOptions :!label _label)
    (CallFunction|RestoreMovementDefaults false)
    (Variables|Default|SetCombatAnimation true)
    (elif (== (Variables|Default|GetStateIndex) 4)
      (Animation|PlayAnimMontage "/Game/FFBLAZE/Enemy/EnemyEmber/EmberairHit.EmberairHit" 1.0 "Land")
      (goto _label)
      (elif (== (Variables|Default|GetStateIndex) 5)
        (Animation|PlayAnimMontage "/Game/FFBLAZE/Enemy/EnemyEmber/Emberdead.Emberdead" 1.0 "Explode")
        (else
          (Animation|PlayAnimMontage "/Game/FFBLAZE/Enemy/EnemyEmber/Land_Montage.Land_Montage" 1.0 "")
          (CallFunction|CanDo true true)
          (CallFunction|ResetAirOptions)
          (CallFunction|StartAnim)
          (CallFunction|RestoreMovementDefaults false)
          (Variables|Default|SetCombatAnimation false)
          (CallFunction|ReleaseBuffer))))))

(event EventHurtAnimation
  (params (AttackerHitbox :type BP%20Hitbox%20Object%20Reference))
  ;[1 1 1] Hurt animation
  (if (Variables|Default|GetInAir)
    (Animation|PlayAnimMontage "/Game/FFBLAZE/Enemy/EnemyEmber/EmberairHit.EmberairHit" 1.0 "")
    (else
      (Animation|PlayAnimMontage "/Game/FFBLAZE/Enemy/EnemyEmber/EmberHit.EmberHit" 1.0 "")))
  (CallFunction|StartAnim)
  (CallFunction|CanDo false true)
  (Variables|Default|SetCanEnemyStep false)
  (Variables|Default|SetStateIndex 4))

(event EventDeathAnimation
  ;[1 1 1] Hurt animation
  (Animation|PlayAnimMontage "/Game/FFBLAZE/Enemy/EnemyEmber/Emberdead.Emberdead" 1.0 "")
  (Variables|Default|SetTargetGravity 0.0)
  (Variables|Default|SetFloatTime 3.0)
  (Utilities|FlowControl|Delay 1.3)
  (for _index (range 0 4)
    (Game|SpawnActorfromClass "/Game/FFBLAZE/Pickups/MoneywaterRefill.MoneywaterRefill_C" (Transformation|GetActorTransform) "Undefined" 0 0))
  (Actor|DestroyActor))

(event EventTick
  (params (DeltaSeconds :type Float%20%28single-precision%29))
  ;[1 1 1] Updater
  (|CallParentFunction DeltaSeconds)
  (CallFunction|ChangeLook)
  (CallFunction|UpdateUI)
  (if (>= (Variables|Default|GetTempTier) 2)
    (Variables|Default|SetTriggerActive true)
    (else
      (Variables|Default|SetTriggerActive false))))

(fn ConstructionScript
  (bind _mesh (Variables|Character|GetMesh))
  (|CallParentFunction)
  (Transformation|AttachComponentToComponent (Variables|Default|GetHurtboxTorso) _mesh "Head" "KeepRelative" "KeepRelative" "KeepRelative" true)
  (Transformation|AttachComponentToComponent (Variables|Default|GetHurtboxLegL) _mesh "Flame_013_L" "KeepRelative" "KeepRelative" "KeepRelative" true)
  (Transformation|AttachComponentToComponent (Variables|Default|GetHurtboxLegR) _mesh "Flame_013_R" "KeepRelative" "KeepRelative" "KeepRelative" true)
  (Transformation|AttachComponentToComponent (Variables|Default|GetRepelSphere) _mesh "Head" "KeepRelative" "KeepRelative" "KeepRelative" true)
  (Variables|Default|SetHurtboxes (Utilities|Array|MakeArray (Variables|Default|GetHurtboxTorso) (Variables|Default|GetHurtboxLegL) (Variables|Default|GetHurtboxLegR))))