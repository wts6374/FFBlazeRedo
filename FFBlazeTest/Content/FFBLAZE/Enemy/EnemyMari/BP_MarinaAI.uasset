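; Marina enemy character that fights the player with combo-style melee, ranged, jump, dodge and teleport moves.
; AI controller action indices become simulated stick directions relative to the locked-on player, so overridden player-style input events can pick directional ground and air moves.
; Each move plays a montage and sets state indices, gravity, velocity and float time.
; Also handles hit and death reactions, the lock-on health widget and health-based TempTier changes.
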(event Custom|UpdateUI
  (bind _healthwidget (Variables|Default|GetHealthWidget))
  ;[1 1 1] Update UI
  (Variables|/Game/FFBLAZE/UI/EnemyHealth.EnemyHealth_C|SetEnemy (Variables|Default|GetUIBar) self)
  (if (Variables|Default|GetIsLockedOn)
    (Rendering|SetVisibility _healthwidget true false)
    (else
      (Rendering|SetVisibility _healthwidget false false))))

(event Custom|StartUI
  ;[1 1 1] Update UI
  (bind _asenemy_health (Utilities|Casting|CastToEnemyHealth (UserInterface|GetUserWidgetObject (Variables|Default|GetHealthWidget))))
  (bind _output_get (Variables|Default|SetUIBar _asenemy_health))
  (Widget|SetVisibility _output_get "Hidden"))

(event Custom|ChargeTimer
  ;[1 1 1] Attack command
  (bind _output_get (Variables|Default|SetLightButton false))
  (|CallParentFunction _output_get)
  (bind _output_get_2 (Variables|Default|SetHeavyButton false))
  (|CallParentFunction _output_get_2))

(event EventBeginPlay
  ;[1 1 1] Initialize
  (|CallParentFunction)
  (bind _asbp_base_character (Utilities|Casting|CastToBP_BaseCharacter (Game|GetPlayerCharacter 0)))
  (Variables|Default|SetLockOnTarget _asbp_base_character)
  (Variables|Default|SetIsLockedOn true)
  (Variables|Default|SetLockonButton true)
  (Variables|Default|SetExtraLives 0))

(event Collision|EventActorBeginOverlap
  (params (OtherActor :type Actor%20Object%20Reference))
  ;[1 1 1] Hurt animation
  (|CallParentFunction OtherActor) ; This node is disabled and will not be called.\nDrag off pins to build functionality.
)

(event EventInputLightAttack
  (params (Pressed :type Boolean))
  (bind _returnvalue (Transformation|GetActorLocation))
  (bind _rotation (CallFunction|CameraYaw))
  (bind _charactermovement (Variables|Character|GetCharacterMovement))
  (bind _charactermovement_2 (Variables|Character|GetCharacterMovement))
  (bind _lockontarget (Variables|Default|GetLockOnTarget))
  (bind _aicontrollerref (Variables|Default|GetAIControllerRef))
  (bind _charactermovement_3 (Variables|Character|GetCharacterMovement))
  (bind _charactermovement_4 (Variables|Character|GetCharacterMovement))
  (bind _charactermovement_5 (Variables|Character|GetCharacterMovement))
  (bind _returnvalue_2 (Transformation|GetActorLocation _lockontarget))
  (bind _aiactionindex (Variables|/Game/StylishCombatKit/AI/AIC_Enemy.AIC_Enemy_C|GetAIActionIndex _aicontrollerref))
  (bind _returnvalue_3 (Math|Vector|GetUnitDirection(Vector) _returnvalue _returnvalue_2))
  (bind (_x _y) (Math|Vector|BreakVector _returnvalue_3))
  (bind _returnvalue_4 (Math|Vector|MakeVector _x _y 0.0))
  (bind _returnvalue_5 (Math|Vector|Normalize _returnvalue_4))
  (bind _returnvalue_6 (Math|Vector|UnrotateVector _returnvalue_5 _rotation))
  (bind _returnvalue_7 (Math|Conversions|ToVector2D(Vector) _returnvalue_6))
  (bind (_x_2 _y_2) (Math|Vector2D|BreakVector2D _returnvalue_7))
  (bind _returnvalue_8 (Math|Vector2D|MakeVector2D _y_2 _x_2))
  ;[1 1 1] Attack command
  (if (Variables|Default|GetCanAttack)
    ;;[1 1 1] Set input vector to simulate directional inputs
    (Variables|Default|SetInputVector (Utilities|Select :Index _aiactionindex :Option%200 (* _returnvalue_8 -1.0) :Option%201 "" :Option%202 _returnvalue_8 :Option%203 ""))
    ;;[1 1 1] Input attack button and hold for specified charge time
    (if (== _aiactionindex 3)
      (CallFunction|StartAnim)
      (CallFunction|CanDo false false)
      (CallFunction|OrientCharacter true true)
      (Animation|PlayAnimMontage "/Game/FFBLAZE/Crystal/Attack/RagingWave.RagingWave" 1.0 "")
      (Variables|Default|SetStateIndex 2)
      (Variables|Default|SetSubStateIndex 4)
      (CallFunction|UpdateRecentMoves -1)
      (else
        (CallFunction|StartAnim)
        (CallFunction|CanDo false false)
        (CallFunction|OrientCharacter true true)
        (switch int (+ (select (== (Variables|Default|GetInputBuffer) 3) (Variables|Default|GetDirectionBuffer) (CallFunction|DirectionalInput)) 1)
          (:0
            ;;;[1 1 1] Back Input: RollingClouds
            (Animation|PlayAnimMontage "/Game/FFBLAZE/Crystal/Attack/Rollingclouds.Rollingclouds" 1.0 "")
            (Variables|Default|SetStateIndex 2)
            (Variables|Default|SetSubStateIndex 7)
            (Variables|/Script/Engine.CharacterMovementComponent|SetGravityScale _charactermovement_4 1.0)
            (Variables|/Script/Engine.MovementComponent|SetVelocity _charactermovement_4 (+ (* (Variables|/Script/Engine.MovementComponent|GetVelocity _charactermovement_4) "0.500000,0.500000,0.000000") "0,0.000000,800.000000"))
            (Variables|Default|SetFloatTime 3.2)
            (CallFunction|UpdateRecentMoves -1))
          (:1
            ;;;[1 1 1] Input attack button and hold for specified charge time
            (if (Variables|Default|GetInAir)
              (bind _returnvalue_9 (Animation|PlayAnimMontage "/Game/FFBLAZE/Crystal/Other/MarinaCancel.MarinaCancel" 1.0 ""))
              (Variables|/Script/Engine.CharacterMovementComponent|SetGravityScale _charactermovement_5 0.3)
              (Variables|/Script/Engine.MovementComponent|SetVelocity _charactermovement_5 (+ (* (Variables|/Script/Engine.MovementComponent|GetVelocity _charactermovement_5) "0.700000,0.700000,0.000000") "0, 0,100.000000"))
              (Variables|Default|SetFloatTime 0.5)
              (Utilities|FlowControl|Delay _returnvalue_9)
              (else
                (bind _returnvalue_10 (Animation|PlayAnimMontage "/Game/FFBLAZE/Crystal/Other/Marina_Anim_root_Taunt_Montage.Marina_Anim_root_Taunt_Montage" 1.0 "None"))
                (Utilities|FlowControl|Delay _returnvalue_10)))
            (switch int (Math|Random|RandomIntegerinRange 0 1)
              (:Default
                (Animation|PlayAnimMontage "/Game/FFBLAZE/Crystal/Attack/RisingTide.RisingTide" 1.0 "" :!label _label)
                (Audio|PlaySound2D "/Game/FFBLAZE/Sound/AttackSFX/atk_axeSwing2.atk_axeSwing2" 0.4 1.0 0.0 0 0)
                (Variables|Default|SetStateIndex 2)
                (Variables|Default|SetSubStateIndex 35)
                (Variables|/Script/Engine.CharacterMovementComponent|SetGravityScale _charactermovement_2 2.0)
                (Variables|/Script/Engine.MovementComponent|SetVelocity _charactermovement_2 (+ (* (Variables|/Script/Engine.MovementComponent|GetVelocity _charactermovement_2) "0.200000,0.200000,0.000000") "0, 0,700.000000"))
                (Variables|Default|SetFloatTime 0.6))
              (:0
                (goto _label))
              (:1
                (bind _returnvalue_11 (Animation|PlayAnimMontage "/Game/FFBLAZE/Crystal/Attack/Spiral.Spiral" 1.0 ""))
                (Audio|PlaySound2D "/Game/FFBLAZE/Sound/AttackSFX/atk_axeSwing3.atk_axeSwing3" 0.4 1.0 0.0 0 0)
                (Variables|Default|SetStateIndex 2)
                (Variables|Default|SetSubStateIndex 12)
                (if (Variables|Default|GetInAir)
                  (Variables|/Script/Engine.CharacterMovementComponent|SetGravityScale _charactermovement 0.0)
                  (Variables|/Script/Engine.MovementComponent|SetVelocity _charactermovement (+ (* (Variables|/Script/Engine.MovementComponent|GetVelocity _charactermovement) "0.700000,0.700000,0.000000") "0, 0, 0")))
                (Variables|Default|SetFloatTime 1.4)))
            (Utilities|FlowControl|Delay _returnvalue_11)
            (CallFunction|UpdateRecentMoves -1))
          (:2
            (if (Variables|Default|GetInAir)
              (Animation|PlayAnimMontage "/Game/FFBLAZE/Crystal/Attack/Harshweather.Harshweather" 1.0 "")
              (Variables|Default|SetStateIndex 2)
              (Variables|Default|SetSubStateIndex 5)
              (else
                (Animation|PlayAnimMontage "/Game/FFBLAZE/Crystal/Attack/Flipback.Flipback" 1.0 "")
                (Variables|Default|SetStateIndex 2)
                (Variables|Default|SetSubStateIndex 6)))
            (Variables|/Script/Engine.CharacterMovementComponent|SetGravityScale _charactermovement_3 2.0)
            (Variables|/Script/Engine.MovementComponent|SetVelocity (Variables|Character|GetCharacterMovement) (+ (* (Variables|/Script/Engine.MovementComponent|GetVelocity _charactermovement_3) "0.500000,0.500000,0.000000") "0, 0,600.000000"))
            (Variables|Default|SetFloatTime 0.8)
            (CallFunction|UpdateRecentMoves -1)))
        (Utilities|Time|SetTimerbyEvent (delegate Custom|ChargeTimer) 0.1)))))

(event EventDeathAnimation
  ;[1 1 1] Hurt animation
  (if (Variables|Default|GetInAir)
    (Animation|PlayAnimMontage "/Game/FFBLAZE/Crystal/Other/Collapse.Collapse" 1.0 "")
    (else
      (Animation|PlayAnimMontage "/Game/FFBLAZE/Crystal/Other/Marina_Anim_root_Dead_Montage.Marina_Anim_root_Dead_Montage" 1.0 "")))
  (Utilities|FlowControl|Delay 5.0)
  (Actor|DestroyActor))

(event EventFlinch
  ;[1 1 1] Hurt animation
  (Animation|PlayAnimMontage "/Game/FFBLAZE/Crystal/Other/Marina_Anim_root_Hit_Montage.Marina_Anim_root_Hit_Montage" 1.5 ""))

(event EventInputJump
  (params (Pressed :type Boolean))
  (bind _rotation (CallFunction|CameraYaw))
  (bind _returnvalue (Transformation|GetActorLocation))
  (bind _aicontrollerref (Variables|Default|GetAIControllerRef))
  (bind _lockontarget (Variables|Default|GetLockOnTarget))
  (bind _charactermovement (Variables|Character|GetCharacterMovement))
  (bind _charactermovement_2 (Variables|Character|GetCharacterMovement))
  (bind _returnvalue_2 (Transformation|GetActorLocation _lockontarget))
  (bind _aiactionindex (Variables|/Game/StylishCombatKit/AI/AIC_Enemy.AIC_Enemy_C|GetAIActionIndex _aicontrollerref))
  (bind _returnvalue_3 (Math|Vector|GetUnitDirection(Vector) _returnvalue _returnvalue_2))
  (bind (_x _y) (Math|Vector|BreakVector _returnvalue_3))
  (bind _returnvalue_4 (Math|Vector|MakeVector _x _y 0.0))
  (bind _returnvalue_5 (Math|Vector|Normalize _returnvalue_4))
  (bind _returnvalue_6 (Math|Vector|UnrotateVector _returnvalue_5 _rotation))
  (bind _returnvalue_7 (Math|Conversions|ToVector2D(Vector) _returnvalue_6))
  (bind (_x_2 _y_2) (Math|Vector2D|BreakVector2D _returnvalue_7))
  (bind _returnvalue_8 (Math|Vector2D|MakeVector2D _y_2 _x_2))
  (bind _returnvalue_9 (* _returnvalue_8 -1.0))
  (bind _returnvalue_10 (Utilities|Select :Index _aiactionindex :Option%200 _returnvalue_9 :Option%201 "" :Option%202 _returnvalue_8 :Option%203 ""))
  ;[1 1 1] JumpCommand
  (if Pressed
    (if (Math|Boolean|ANDBoolean (Variables|Default|GetCanMove) (> (Variables|Default|GetTempTier) 0) (< (Variables|Default|GetAirJumpsUsed) 1))
      (if (Variables|Default|GetInAir)
        (Variables|Default|SetInputVector _returnvalue_10)
        (bind _output_get (Variables|Default|SetAirJumpsUsed (- (Variables|Default|GetAirJumpsUsed) -1)))
        (switch int _output_get
          (:Default
            (CallFunction|OrientCharacter (or (<= (Math|Vector2D|Vector2DLength (Variables|Default|GetInputVector)) (Variables|Default|GetWalkThreshold)) (!= (CallFunction|DirectionalInput) 0)) false :!label _label)
            (CallFunction|StartAnim)
            (CallFunction|CanDo false true)
            (Animation|PlayAnimMontage "/Game/FFBLAZE/Crystal/Movement/MarinaDodge.MarinaDodge" 1.0 "None")
            (Audio|PlaySound2D "/Game/FFBLAZE/Sound/dash.dash" 0.5 0.8 0.0 0 0)
            (Math|Integer|IncrementInt (Variables|Default|GetAirDashesUsed)
              (:%20%20
                (Variables|/Script/Engine.CharacterMovementComponent|SetGravityScale _charactermovement_2 0.0)
                (Variables|Default|SetFloatTime 0.5)
                (Variables|/Script/Engine.MovementComponent|SetVelocity _charactermovement_2 "2.000000,2.000000,1.000000")
                (Variables|Default|SetStateIndex 1)
                (Variables|Default|SetSubStateIndex 1)
                (CallFunction|SetInvinciblity true))))
          (:0
            ;;[1 1 1] Teleport
            (if (or (< (Variables|Default|GetAirTeleportsUsed) 1) (not (Variables|Default|GetInAir))) :!label _label_2
              (CallFunction|StartAnim)
              (CallFunction|RestoreMovementDefaults true)
              (CallFunction|OrientCharacter true false)
              (Variables|/Script/Engine.MovementComponent|SetVelocity _charactermovement (+ (* (Transformation|GetActorForwardVector) 5e+01) "0, 0,100.000000"))
              (Variables|Default|SetFloatTime 0.2)
              (Variables|/Script/Engine.CharacterMovementComponent|SetGravityScale _charactermovement 2.0)
              (Variables|Default|SetStateIndex 1)
              (Variables|Default|SetSubStateIndex 10)
              (CallFunction|SetInvinciblity true)
              (if (Variables|Default|GetInAir)
                (Math|Integer|IncrementInt (Variables|Default|GetAirTeleportsUsed)
                  (:%20%20
                    _)))
              (Animation|PlayAnimMontage "/Game/FFBLAZE/Crystal/Movement/MariWarp.MariWarp" 1.0 "Start")
              (Variables|Default|SetInputBuffer 0)
              (CallFunction|CanDo false true)
              (Effects|SpawnEmitteratLocation "/Game/StylishCombatKit/VFX/ParticleSystems/P_TeleportBlue.P_TeleportBlue" (Transformation|GetActorLocation))
              (Variables|Default|SetDodging true)))
          (:1
            (goto _label))
          (:2
            (goto _label)))
        (else
          ;;[1 1 1] Set input vector to simulate directional inputs
          (Variables|Default|SetInputVector _returnvalue_10)
          ;;[1 1 1] Input attack button and hold for specified charge time
          (if (== _aiactionindex 3)
            (Variables|Default|SetInputVector "")
            (Variables|Default|SetAirJumpsUsed (- (Variables|Default|GetAirJumpsUsed) -1))
            (goto _label_2)
            (else
              (CallFunction|StartAnim)
              (CallFunction|CanDo false false)
              (CallFunction|OrientCharacter true true)
              (switch int (+ (select (== (Variables|Default|GetInputBuffer) 3) (Variables|Default|GetDirectionBuffer) (CallFunction|DirectionalInput)) 1)
                (:Default
                  (CallFunction|JumpEvent true "/Game/FFBLAZE/Crystal/Movement/Marina_Anim_root_jump_Montage.Marina_Anim_root_jump_Montage" "/Game/FFBLAZE/Crystal/Movement/Marina_Anim_root_jump_Forward_Montage.Marina_Anim_root_jump_Forward_Montage" "/Game/FFBLAZE/Crystal/Movement/Marina_Anim_root_jump_Back_Montage.Marina_Anim_root_jump_Back_Montage" :!label _label_3))
                (:0
                  (CallFunction|OrientCharacter (or (<= (Math|Vector2D|Vector2DLength (Variables|Default|GetInputVector)) (Variables|Default|GetWalkThreshold)) (!= (CallFunction|DirectionalInput) 0)) false)
                  (CallFunction|StartAnim)
                  (CallFunction|CanDo false true)
                  (Animation|PlayAnimMontage "/Game/FFBLAZE/Crystal/Movement/MarinaDodge.MarinaDodge" 1.0 "None")
                  (Audio|PlaySound2D "/Game/FFBLAZE/Sound/dash.dash" 0.5 0.8 0.0 0 0)
                  (Variables|Default|SetStateIndex 1)
                  (Variables|Default|SetSubStateIndex 1))
                (:1
                  (goto _label_3))
                (:2
                  (goto _label_3))))))))
    (else
      (Variables|Default|SetJumpTimer 0.0))))

(event EventInputHeavyAttack
  (params (Pressed :type Boolean))
  (bind _rotation (CallFunction|CameraYaw))
  (bind _returnvalue (Transformation|GetActorLocation))
  (bind _lockontarget (Variables|Default|GetLockOnTarget))
  (bind _charactermovement (Variables|Character|GetCharacterMovement))
  (bind _charactermovement_2 (Variables|Character|GetCharacterMovement))
  (bind _charactermovement_3 (Variables|Character|GetCharacterMovement))
  (bind _charactermovement_4 (Variables|Character|GetCharacterMovement))
  (bind _charactermovement_5 (Variables|Character|GetCharacterMovement))
  (bind _charactermovement_6 (Variables|Character|GetCharacterMovement))
  (bind _charactermovement_7 (Variables|Character|GetCharacterMovement))
  (bind _charactermovement_8 (Variables|Character|GetCharacterMovement))
  (bind _inair (Variables|Default|GetInAir))
  (bind _aicontrollerref (Variables|Default|GetAIControllerRef))
  (bind _returnvalue_2 (Transformation|GetActorLocation _lockontarget))
  (bind _aiactionindex (Variables|/Game/StylishCombatKit/AI/AIC_Enemy.AIC_Enemy_C|GetAIActionIndex _aicontrollerref))
  (bind _returnvalue_3 (Math|Vector|GetUnitDirection(Vector) _returnvalue _returnvalue_2))
  (bind (_x _y) (Math|Vector|BreakVector _returnvalue_3))
  (bind _returnvalue_4 (Math|Vector|MakeVector _x _y 0.0))
  (bind _returnvalue_5 (Math|Vector|Normalize _returnvalue_4))
  (bind _returnvalue_6 (Math|Vector|UnrotateVector _returnvalue_5 _rotation))
  (bind _returnvalue_7 (Math|Conversions|ToVector2D(Vector) _returnvalue_6))
  (bind (_x_2 _y_2) (Math|Vector2D|BreakVector2D _returnvalue_7))
  (bind _returnvalue_8 (Math|Vector2D|MakeVector2D _y_2 _x_2))
  ;[1 1 1] Attack command
  (if (Variables|Default|GetCanAttack)
    ;;[1 1 1] Set input vector to simulate directional inputs
    (Variables|Default|SetInputVector (Utilities|Select :Index _aiactionindex :Option%200 (* _returnvalue_8 -1.0) :Option%201 "" :Option%202 _returnvalue_8 :Option%203 ""))
    ;;[1 1 1] Input attack button and hold for specified charge time
    (if (== _aiactionindex 3)
      (CallFunction|StartAnim)
      (CallFunction|CanDo false false)
      (CallFunction|OrientCharacter true true)
      (Animation|PlayAnimMontage "/Game/FFBLAZE/Crystal/Attack/Hail.Hail" 1.0 "")
      (Variables|Default|SetStateIndex 2)
      (Variables|Default|SetSubStateIndex 30)
      (Variables|/Script/Engine.CharacterMovementComponent|SetGravityScale _charactermovement 0.2)
      (Variables|/Script/Engine.MovementComponent|SetVelocity _charactermovement (+ (* (Variables|/Script/Engine.MovementComponent|GetVelocity _charactermovement) "0.700000,0.700000,0.000000") "0, 0,100.000000"))
      (Variables|Default|SetFloatTime 0.5)
      (CallFunction|UpdateRecentMoves -1)
      (else
        (CallFunction|StartAnim)
        (CallFunction|CanDo false false)
        (CallFunction|OrientCharacter true true)
        (switch int (+ (select (== (Variables|Default|GetInputBuffer) 3) (Variables|Default|GetDirectionBuffer) (CallFunction|DirectionalInput)) 1)
          (:0
            (if (Variables|Default|GetInAir)
              ;;;[1 1 1] Forward Input: Windshift (ground only)
              (Animation|PlayAnimMontage "/Game/FFBLAZE/Crystal/Attack/Dualshock.Dualshock" 1.1 "")
              (Variables|Default|SetStateIndex 2)
              (Variables|Default|SetSubStateIndex 23)
              (Variables|/Script/Engine.CharacterMovementComponent|SetGravityScale _charactermovement_5 2.0)
              (Variables|/Script/Engine.MovementComponent|SetVelocity _charactermovement_5 (+ (* (Variables|/Script/Engine.MovementComponent|GetVelocity _charactermovement_5) "0.500000,0.500000,0.000000") "0, 0,300.000000"))
              (Variables|Default|SetFloatTime 0.3)
              (else
                (Animation|PlayAnimMontage "/Game/FFBLAZE/Crystal/Attack/Windshift.Windshift" 1.4 "")
                (Variables|Default|SetStateIndex 2)
                (Variables|Default|SetSubStateIndex 22)
                (Variables|/Script/Engine.CharacterMovementComponent|SetGravityScale _charactermovement_6 2.0)
                (Variables|/Script/Engine.MovementComponent|SetVelocity _charactermovement_6 (+ (* (Variables|/Script/Engine.MovementComponent|GetVelocity _charactermovement_6) "0.500000,0.500000,0.000000") "0, 0,100.000000"))
                (Variables|Default|SetFloatTime 0.3)))
            (CallFunction|UpdateRecentMoves -1)
            ;[1 1 1] Attack command
            (Utilities|Time|SetTimerbyEvent (delegate Custom|ChargeTimer) 0.1 :!label _label))
          (:1
            (bind _returnvalue_9 (Animation|PlayAnimMontage "/Game/FFBLAZE/Crystal/Other/MarinaCancel.MarinaCancel" 1.0 ""))
            (Variables|/Script/Engine.CharacterMovementComponent|SetGravityScale _charactermovement_7 0.3)
            (Variables|/Script/Engine.MovementComponent|SetVelocity _charactermovement_7 (+ (* (Variables|/Script/Engine.MovementComponent|GetVelocity _charactermovement_7) "0.700000,0.700000,0.000000") "0, 0,100.000000"))
            (Variables|Default|SetFloatTime 0.5)
            (Utilities|FlowControl|Delay _returnvalue_9)
            (for _index (range 0 9)
              (if _inair
                (CallFunction|CanDo _inair true)
                (if (Variables|Default|GetisBlasting)
                  _
                  (else
                    (CallFunction|RestoreMovementDefaults true :!label _label_2)))
                (else
                  (CallFunction|CanDo true true)
                  (goto _label_2)))
              (Variables|Default|SetStateIndex 9)
              (Variables|Default|SetSubStateIndex 1)
              (CallFunction|GetPitch true true)
              (Animation|PlayAnimMontage "/Game/FFBLAZE/Crystal/Water/MariFire.MariFire" 1.0 "None")
              (if (Variables|Default|GetInAir)
                (Variables|/Script/Engine.CharacterMovementComponent|SetGravityScale _charactermovement_8 0.5)
                (Variables|/Script/Engine.MovementComponent|SetVelocity (Variables|Character|GetCharacterMovement) (+ (Variables|/Script/Engine.MovementComponent|GetVelocity _charactermovement_8) "0.000000, 0,-0.100000")))
              (CallFunction|UpdateRecentMoves 0)
              (goto _label))
            (CallFunction|StartAnim)
            (CallFunction|CanDo false true)
            (CallFunction|GetPitch true true)
            (CallFunction|RestoreMovementDefaults false)
            (CallFunction|ReleaseBuffer)
            (bind _returnvalue_10 (Animation|PlayAnimMontage "/Game/FFBLAZE/Crystal/Water/MariBurst.MariBurst" 1.2 ""))
            (Audio|PlaySound2D "/Game/StarterContent/Audio/Explosion_Cue.Explosion_Cue" 0.2 1.0 0.0 0 0 false)
            (Variables|Default|SetStateIndex 9)
            (Variables|Default|SetSubStateIndex 12)
            (Variables|/Script/Engine.CharacterMovementComponent|SetGravityScale _charactermovement_3 6.0)
            (Variables|/Script/Engine.MovementComponent|SetVelocity _charactermovement_3 (+ (* (Variables|/Script/Engine.MovementComponent|GetVelocity _charactermovement_3) "0.700000,0.700000,0.000000") "0, 0,700.000000"))
            (Variables|Default|SetFloatTime 0.8)
            (Variables|Default|SetJumpTimer 0.1)
            (Utilities|FlowControl|Delay _returnvalue_10)
            (CallFunction|OrientCharacter (or (<= (Math|Vector2D|Vector2DLength (Variables|Default|GetInputVector)) (Variables|Default|GetWalkThreshold)) (!= (CallFunction|DirectionalInput) 0)) false)
            (CallFunction|StartAnim)
            (CallFunction|CanDo false true)
            (Animation|PlayAnimMontage "/Game/FFBLAZE/Crystal/Movement/MarinaDodge.MarinaDodge" 1.0 "None")
            (Audio|PlaySound2D "/Game/FFBLAZE/Sound/dash.dash" 0.5 0.8 0.0 0 0)
            (Math|Integer|IncrementInt (Variables|Default|GetAirDashesUsed)
              (:%20%20
                (Variables|/Script/Engine.CharacterMovementComponent|SetGravityScale _charactermovement_4 0.0)
                (Variables|Default|SetFloatTime 0.3)
                (Variables|/Script/Engine.MovementComponent|SetVelocity _charactermovement_4 "2.000000,2.000000,0.000000")
                (CallFunction|CanDo (Variables|Default|GetInAir) true)
                (Variables|Default|SetJumpTimer 0.1))))
          (:2
            (if (Variables|Default|GetInAir)
              (Animation|PlayAnimMontage "/Game/FFBLAZE/Crystal/Attack/Acidrain.Acidrain" 1.0 "")
              (Variables|Default|SetStateIndex 2)
              (Variables|Default|SetSubStateIndex 25)
              (Variables|/Script/Engine.CharacterMovementComponent|SetGravityScale _charactermovement_2 1.0)
              (Variables|/Script/Engine.MovementComponent|SetVelocity _charactermovement_2 (+ (* (Variables|/Script/Engine.MovementComponent|GetVelocity _charactermovement_2) "0.500000,0.500000,0.000000") "2000.000000, 0,600.000000"))
              (Variables|Default|SetFloatTime 2.0)
              (else
                (Animation|PlayAnimMontage "/Game/FFBLAZE/Crystal/Attack/Rainfall.Rainfall" 1.0 "")
                (Variables|Default|SetStateIndex 2)
                (Variables|Default|SetSubStateIndex 21)))
            (Variables|Default|SetHeavyCharge (Variables|Default|GetHeavyButton))
            (Variables|Default|SetHeavyChargeLevel -1)
            (CallFunction|UpdateRecentMoves -1)))))))

(event EventAdjustTemperature
  (params (WaterIntake :type Float%20%28single-precision%29))
  ;[1 1 1] Hurt animation
  (if (<= (Variables|Default|GetHealth) (- (Variables|Default|GetMaxHealth) 2e+02))
    (Variables|Default|SetTempTier 2))
  (if (<= (Variables|Default|GetHealth) (/ (Variables|Default|GetMaxHealth) 5.0))
    (Variables|Default|SetTempTier 3)
    (if true
      (Utilities|Time|SetGlobalTimeDilation (Math|Conversions|ToFloat(Boolean) (< (Variables|Default|GetTempTier) 2))))))

(event EventGetHit
  (params (HitData :type Struct%20Hit%20Data%20Structure) (AttackerHitbox :type BP%20Hitbox%20Object%20Reference) (HitResult :type Hit%20Result%20Structure))
  ;[1 1 1] Hurt animation
  ;;[1 1 1] Special hit effects
  (|CallParentFunction HitData AttackerHitbox HitResult)
  (Variables|/Script/Engine.CharacterMovementComponent|SetGravityScale (Variables|Character|GetCharacterMovement) 5.0)
  (Variables|Default|SetTriggerActive false))

(event EventSpecialAttacks
  ;[1 1 1] Updater
  (Variables|Default|SetTriggerActive false))

(event EventTick
  (params (DeltaSeconds :type Float%20%28single-precision%29))
  ;[1 1 1] Updater
  (|CallParentFunction DeltaSeconds)
  (CallFunction|UpdateUI)
  (CallFunction|SpecialAttacks))

(event EventHurtAnimation
  (params (AttackerHitbox :type BP%20Hitbox%20Object%20Reference))
  (bind _ownercharacter (Variables|/Game/StylishCombatKit/Misc/BP_Hitbox.BP_Hitbox_C|GetOwnerCharacter AttackerHitbox))
  ;[1 1 1] Hurt animation
  (Variables|Default|SetDodgeRecharge 0.0)
  (if (Variables|Default|GetInAir)
    (Animation|PlayAnimMontage "/Game/FFBLAZE/Crystal/Other/Marina_Anim_root_AirHit_Montage.Marina_Anim_root_AirHit_Montage" 2.0 "")
    (else
      (Animation|PlayAnimMontage (select (or (>= (Variables|/Game/StylishCombatKit/Main/BP_BaseCharacter.BP_BaseCharacter_C|GetLightChargeLevel _ownercharacter) 1) (>= (Variables|/Game/StylishCombatKit/Main/BP_BaseCharacter.BP_BaseCharacter_C|GetHeavyChargeLevel _ownercharacter) 1)) "/Game/FFBLAZE/Crystal/Other/Marina_Anim_root_Hit_Montage.Marina_Anim_root_Hit_Montage" "/Game/FFBLAZE/Crystal/Other/Marina_Anim_root_Hit_Montage.Marina_Anim_root_Hit_Montage") 2.0 "")))
  (CallFunction|StartAnim)
  (CallFunction|CanDo false true)
  (Variables|Default|SetCanEnemyStep false)
  (Variables|Default|SetStateIndex 4))

(fn ConstructionScript
  (|CallParentFunction))