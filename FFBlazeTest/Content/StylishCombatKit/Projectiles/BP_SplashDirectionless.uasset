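; Water splash projectile for the combat kit that carries a damaging, launching hitbox with a cooling effect and no aiming of its own.
; Initialize spawns a small spherical BP_Hitbox on its capsule, fills in the water hit data and activates it; the lock-on branch leaves velocity unchanged.
; Tick runs the hit-reset check and counts Duration down using custom time dilation, destroying the actor at zero; the WaitPeriod countdown triggers nothing.
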(event EventBeginPlay
  (|CallParentFunction) ; This node is disabled and will not be called.\nDrag off pins to build functionality.
)

(event Collision|EventActorBeginOverlap
  (params (OtherActor :type Actor%20Object%20Reference)))

(event EventTick
  (params (DeltaSeconds :type Float%20%28single-precision%29))
  (bind _customtimedilation (Variables|Default|GetCustomTimeDilation))
  (bind _returnvalue (* DeltaSeconds _customtimedilation))
  ;[1 1 1] Update values on tick
  (|CallParentFunction DeltaSeconds)
  (CallFunction|ResetHitsCheck)
  (if (> (Variables|Default|GetDuration) 0.0)
    (Variables|Default|SetDuration (Math|Float|Clamp(Float) (- (Variables|Default|GetDuration) _returnvalue) 0.0 (Variables|Default|GetDuration))))
  (if (== (Variables|Default|GetDuration) 0.0)
    (CallFunction|Destroy)
    (else
      (Variables|Default|SetWaitPeriod (Math|Float|Clamp(Float) (- (Variables|Default|GetWaitPeriod) _returnvalue) 0.0 (Variables|Default|GetWaitPeriod)))
      (if (== (Variables|Default|GetWaitPeriod) 0.0)
        _))))

(event EventInitialize
  (bind _charactermovement (Variables|Character|GetCharacterMovement))
  ;[1 1 1] Initialize
  (|CallParentFunction)
  (bind _returnvalue (Game|SpawnActorfromClass "/Game/StylishCombatKit/Misc/BP_Hitbox.BP_Hitbox_C" (Transformation|GetActorTransform) "AlwaysSpawn" 0 0))
  (Variables|/Game/StylishCombatKit/Misc/BP_Hitbox.BP_Hitbox_C|SetOwnerCharacter _returnvalue self)
  (Transformation|AttachComponentToComponent _returnvalue (Variables|Default|GetCapsuleComponent) "None" "KeepWorld" "KeepWorld" "KeepWorld" true)
  (Utilities|Array|Add (Variables|Default|GetHitboxes) _returnvalue)
  (Variables|/Game/StylishCombatKit/Misc/BP_Hitbox.BP_Hitbox_C|SetHitData _returnvalue (Utilities|Struct|MakeStruct_HitData 0 "1000.000000,0.000000,1000.000000" 2e+01 2 0.5 0.02 0.0 true 75.0))
  (Components|Sphere|SetSphereRadius (Variables|/Game/StylishCombatKit/Misc/BP_Hitbox.BP_Hitbox_C|GetHitbox _returnvalue) 6e+01 true)
  (Transformation|SetActorRelativeLocation _returnvalue)
  (Default|Activate _returnvalue true)
  (if (and (Variables|/Game/StylishCombatKit/Main/BP_BaseCharacter.BP_BaseCharacter_C|GetIsLockedOn (Variables|Default|GetOwnerCharacter)) (Utilities|IsValid (Variables|/Game/StylishCombatKit/Main/BP_BaseCharacter.BP_BaseCharacter_C|GetLockOnTarget (Variables|Default|GetOwnerCharacter))))
    (bind _output_get (Variables|/Script/Engine.MovementComponent|SetVelocity _charactermovement (Variables|/Script/Engine.MovementComponent|GetVelocity _charactermovement)))
    (Variables|Default|SetPreviousFrameVelocity _output_get)))

(fn ConstructionScript
  (|CallParentFunction))