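; BP_Shop is an interactable shop that toggles a shopping menu for the BP_BaseCharacter using it.
; On Interact it creates and caches the ShoppingMenu widget if needed, then uses the game's paused state as the toggle.
; Opening pauses the game, shows the cursor and hands the menu to the player.
; Closing unpauses, restores game-only input, plays the purchase sound and refreshes the player's moves.
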(event EventInteract
  (params (Player :type Character%20Object%20Reference))
  (bind _returnvalue (Game|GetPlayerController 0))
  (Utilities|IsValid Player
    (:Is%20Valid
      (bind _asbp_base_character (Utilities|Casting|CastToBP_BaseCharacter Player))
      (Variables|Default|SetPlayer _asbp_base_character)
      (Utilities|IsValid (Variables|Default|GetShopmenu%20Ref)
        (:Is%20Valid
          _)
        (:Is%20Not%20Valid
          (bind _returnvalue_2 (UserInterface|CreateWidget "/Game/FFBLAZE/UI/ShoppingMenu.ShoppingMenu_C"))
          (Variables|Default|SetShopmenu%20Ref _returnvalue_2)))
      (if (Game|IsGamePaused)
        (Widget|RemovefromParent (Variables|Default|GetShopmenu%20Ref))
        (Game|SetGamePaused false)
        (Variables|/Script/Engine.PlayerController|SetbShowMouseCursor _returnvalue false)
        (Input|SetInputModeGameOnly _returnvalue)
        (Audio|PlaySoundatLocation "/Game/FFBLAZE/Sound/ShopOrCurrencySFX/purchased_sound.purchased_sound" (Variables|/Script/Engine.SceneComponent|GetRelativeLocation (Variables|Default|GetBox)) "0, 0, 0" 0.5 1.0 0.0 0 0 0)
        (Default|RefreshMoves (Variables|Default|GetPlayer))
        (else
          (UserInterface|Viewport|AddtoViewport (Variables|Default|GetShopmenu%20Ref) 0)
          (Game|SetGamePaused true)
          (Variables|/Script/Engine.PlayerController|SetbShowMouseCursor _returnvalue true)
          (Input|SetInputModeGameandUI _returnvalue (Variables|Default|GetShopmenu%20Ref) "LockInFullscreen" false)
          (Variables|/Game/StylishCombatKit/Main/BP_BaseCharacter.BP_BaseCharacter_C|SetShopMenu (Variables|Default|GetPlayer) (Variables|Default|GetShopmenu%20Ref)))))))

(fn ConstructionScript)