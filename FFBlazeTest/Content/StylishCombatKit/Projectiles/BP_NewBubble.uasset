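; BP_NewBubble is a bubble projectile in the Stylish Combat Kit that flies forward and delivers water, cooling hits with an upward launch.
; On initialization it attaches a small spherical BP_Hitbox and sets flying movement along its forward vector.
; Each tick it redirects velocity along the owner-to-lock-on-target direction, keeping speed, and resets hit checks.
; It destroys itself at zero Duration, though the countdown subtracts zero as wired.
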(event EventTick
  (params (DeltaSeconds :type Float%20%28single-precision%29))
  (bind _ownercharacter (Variables|Default|GetOwnerCharacter))
  (bind _ownercharacter_2 (Variables|Default|GetOwnerCharacter))
  (bind _charactermovement (Variables|Character|GetCharacterMovement))
  ;[1 1 1] Initialize
  (|CallParentFunction DeltaSeconds)
  (if (and (Variables|/Game/StylishCombatKit/Main/BP_BaseCharacter.BP_BaseCharacter_C|GetIsLockedOn _ownercharacter_2) (Utilities|IsValid (Variables|/Game/StylishCombatKit/Main/BP_BaseCharacter.BP_BaseCharacter_C|GetLockOnTarget _ownercharacter_2)))
    (bind _output_get (Variables|/Script/Engine.MovementComponent|SetVelocity _charactermovement (* (Math|Vector|GetUnitDirection(Vector) (Transformation|GetActorLocation _ownercharacter) (Transformation|GetActorLocation (Variables|/Game/StylishCombatKit/Main/BP_BaseCharacter.BP_BaseCharacter_C|GetLockOnTarget _ownercharacter))) (Math|Vector|VectorLength (Variables|/Script/Engine.MovementComponent|GetVelocity _charactermovement)))))
    (Variables|Default|SetPreviousFrameVelocity _output_get))
  ;[1 1 1] Update values on tick
  (CallFunction|ResetHitsCheck)
  (if (> (Variables|Default|GetDuration) 0.0)
    (Variables|Default|SetDuration (Math|Float|Clamp(Float) (- (Variables|Default|GetDuration) (* 0.0 (Variables|Default|GetCustomTimeDilation))) 0.0 (Variables|Default|GetDuration))))
  (if (== (Variables|Default|GetDuration) 0.0)
    (CallFunction|Destroy)))

(event EventInitialize
  (bind _charactermovement (Variables|Character|GetCharacterMovement))
  ;[1 1 1] Initialize
  (|CallParentFunction)
  (bind _returnvalue (Game|SpawnActorfromClass "/Game/StylishCombatKit/Misc/BP_Hitbox.BP_Hitbox_C" (Transformation|GetActorTransform) "AlwaysSpawn" 0 0))
  (Variables|/Game/StylishCombatKit/Misc/BP_Hitbox.BP_Hitbox_C|SetOwnerCharacter _returnvalue self)
  (Transformation|AttachComponentToComponent _returnvalue (Variables|Default|GetCapsuleComponent) "None" "KeepWorld" "KeepWorld" "KeepWorld" true)
  (Utilities|Array|Add (Variables|Default|GetHitboxes) _returnvalue)
  (Components|Sphere|SetSphereRadius (Variables|/Game/StylishCombatKit/Misc/BP_Hitbox.BP_Hitbox_C|GetHitbox _returnvalue) 8.0 true)
  (Variables|/Game/StylishCombatKit/Misc/BP_Hitbox.BP_Hitbox_C|SetHitData _returnvalue (Utilities|Struct|MakeStruct_HitData 1 "0.000000,0.000000,700.000000" 1e+01 2 0.001 0.1 0.0 true 7e+01))
  (Default|Activate _returnvalue true)
  (Pawn|Components|CharacterMovement|SetMovementMode (Variables|Character|GetCharacterMovement) "MOVE_Flying" 0)
  (bind _output_get (Variables|/Script/Engine.MovementComponent|SetVelocity (Variables|Character|GetCharacterMovement) (* (Transformation|GetActorForwardVector) (Variables|Default|GetSpeed))))
  (Variables|Default|SetPreviousFrameVelocity _output_get)
  (if (and (Variables|/Game/StylishCombatKit/Main/BP_BaseCharacter.BP_BaseCharacter_C|GetIsLockedOn (Variables|Default|GetOwnerCharacter)) (Utilities|IsValid (Variables|/Game/StylishCombatKit/Main/BP_BaseCharacter.BP_BaseCharacter_C|GetLockOnTarget (Variables|Default|GetOwnerCharacter))))
    (bind _output_get_2 (Variables|/Script/Engine.MovementComponent|SetVelocity _charactermovement (* (Math|Vector|GetUnitDirection(Vector) (Transformation|GetActorLocation (Variables|Default|GetOwnerCharacter)) (Transformation|GetActorLocation (Variables|/Game/StylishCombatKit/Main/BP_BaseCharacter.BP_BaseCharacter_C|GetLockOnTarget (Variables|Default|GetOwnerCharacter)))) (Math|Vector|VectorLength (Variables|/Script/Engine.MovementComponent|GetVelocity _charactermovement)))))
    (Variables|Default|SetPreviousFrameVelocity _output_get_2))
  ;[1 1 1] Update values on tick
  (CallFunction|ResetHitsCheck)
  (if (> (Variables|Default|GetDuration) 0.0)
    (Variables|Default|SetDuration (Math|Float|Clamp(Float) (- (Variables|Default|GetDuration) (* 0.0 (Variables|Default|GetCustomTimeDilation))) 0.0 (Variables|Default|GetDuration))))
  (if (== (Variables|Default|GetDuration) 0.0)
    (CallFunction|Destroy)))

(fn ConstructionScript
  (|CallParentFunction))