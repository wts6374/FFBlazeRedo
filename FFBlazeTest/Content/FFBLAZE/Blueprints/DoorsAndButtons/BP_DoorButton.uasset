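; BP_DoorButton is an interactable button that opens the doors linked to it by a shared number.
; On Interact, it searches all BP_Door actors in the level and calls OpenDoor with the interacting player on each whose DoorValue equals its ButtonValue.
; Each match also turns the button's cube red and plays a coin-collect sound, positioned using the box component's relative, not world, location.
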(event EventInteract
  (params (Player :type Character%20Object%20Reference))
  (bind _outactors (Actor|GetAllActorsOfClass "/Game/FFBLAZE/Blueprints/DoorsAndButtons/BP_Door.BP_Door_C"))
  (bind _array_element (Utilities|Array|ForEachLoopwithBreak _outactors)
    (:LoopBody
      (if (== (Variables|/Game/FFBLAZE/Blueprints/DoorsAndButtons/BP_Door.BP_Door_C|GetDoor%20Value _array_element) (Variables|Default|GetButton%20Value))
        (Default|OpenDoor _array_element Player)
        (Rendering|Material|SetMaterial (Variables|Default|GetCube) 0 "/Game/FFBLAZE/TexturesAndMaterials/Red.Red")
        (Audio|PlaySoundatLocation "/Game/FFBLAZE/Sound/ShopOrCurrencySFX/collected_coin_sound.collected_coin_sound" (Variables|/Script/Engine.SceneComponent|GetRelativeLocation (Variables|Default|GetBox)) "0, 0, 0" 0.5 1.0 0.0 0 0 0)))))

(fn ConstructionScript)