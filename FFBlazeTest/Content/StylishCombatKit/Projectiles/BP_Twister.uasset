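; BP_Twister is a character-based combat projectile that creates a water-type damaging area around its owner.
; On initialize it attaches a large spherical BP_Hitbox with launch and hit-stop data, then sets flying movement with forward velocity.
; Each tick it snaps to the owner's location and runs the hit-reset check.
; It destroys itself at zero Duration, though the countdown subtracts zero, so Duration never decreases here.
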(event EventTick
  (params (DeltaSeconds :type Float%20%28single-precision%29))
  ;[1 1 1] Initialize
  (|CallParentFunction DeltaSeconds)
  (Transformation|SetActorLocation (Transformation|GetActorLocation (Variables|Default|GetOwnerCharacter)) false false)
  ;[1 1 1] Update values on tick
  (CallFunction|ResetHitsCheck)
  (if (> (Variables|Default|GetDuration) 0.0)
    (Variables|Default|SetDuration (Math|Float|Clamp(Float) (- (Variables|Default|GetDuration) (* 0.0 (Variables|Default|GetCustomTimeDilation))) 0.0 (Variables|Default|GetDuration))))
  (if (== (Variables|Default|GetDuration) 0.0)
    (CallFunction|Destroy)))

(event EventInitialize
  ;[1 1 1] Initialize
  (|CallParentFunction)
  (bind _returnvalue (Game|SpawnActorfromClass "/Game/StylishCombatKit/Misc/BP_Hitbox.BP_Hitbox_C" (Transformation|GetActorTransform) "AlwaysSpawn" 0 0))
  (Variables|/Game/StylishCombatKit/Misc/BP_Hitbox.BP_Hitbox_C|SetOwnerCharacter _returnvalue self)
  (Transformation|AttachComponentToComponent _returnvalue (Variables|Default|GetCapsuleComponent) "None" "KeepWorld" "KeepWorld" "KeepWorld" true)
  (Utilities|Array|Add (Variables|Default|GetHitboxes) _returnvalue)
  (Components|Sphere|SetSphereRadius (Variables|/Game/StylishCombatKit/Misc/BP_Hitbox.BP_Hitbox_C|GetHitbox _returnvalue) 3e+02 true)
  (Variables|/Game/StylishCombatKit/Misc/BP_Hitbox.BP_Hitbox_C|SetHitData _returnvalue (Utilities|Struct|MakeStruct_HitData 0 "-400.000000,0.000000,200.000000" 4.0 2 0.1 0.1 0.0 true 4e+01))
  (Default|Activate _returnvalue true)
  (Pawn|Components|CharacterMovement|SetMovementMode (Variables|Character|GetCharacterMovement) "MOVE_Flying" 0)
  (bind _output_get (Variables|/Script/Engine.MovementComponent|SetVelocity (Variables|Character|GetCharacterMovement) (* (Transformation|GetActorForwardVector) (Variables|Default|GetSpeed))))
  (Variables|Default|SetPreviousFrameVelocity _output_get)
  (Transformation|SetActorLocation (Transformation|GetActorLocation (Variables|Default|GetOwnerCharacter)) false false)
  ;[1 1 1] Update values on tick
  (CallFunction|ResetHitsCheck)
  (if (> (Variables|Default|GetDuration) 0.0)
    (Variables|Default|SetDuration (Math|Float|Clamp(Float) (- (Variables|Default|GetDuration) (* 0.0 (Variables|Default|GetCustomTimeDilation))) 0.0 (Variables|Default|GetDuration))))
  (if (== (Variables|Default|GetDuration) 0.0)
    (CallFunction|Destroy)))

(fn ConstructionScript
  (|CallParentFunction))