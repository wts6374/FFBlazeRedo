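; BP_CounterProjectile is a character-based projectile in StylishCombatKit that flies forward carrying a damaging hitbox.
; On Initialize it spawns a BP_Hitbox, attaches it to its capsule, sizes the sphere and fills HitData with damage, upward launch and meter gain before activating it.
; It then switches CharacterMovement to Flying and sets velocity along the actor's forward vector, caching it as PreviousFrameVelocity.
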(event EventBeginPlay
  (|CallParentFunction))

(event EventTick
  (params (DeltaSeconds :type Float%20%28single-precision%29))
  (|CallParentFunction DeltaSeconds))

(event EventInitialize
  ;[1 1 1] Initialize
  (|CallParentFunction)
  (bind _returnvalue (Game|SpawnActorfromClass "/Game/StylishCombatKit/Misc/BP_Hitbox.BP_Hitbox_C" (Transformation|GetActorTransform) "AlwaysSpawn" 0 0))
  (Variables|/Game/StylishCombatKit/Misc/BP_Hitbox.BP_Hitbox_C|SetOwnerCharacter _returnvalue self)
  (Transformation|AttachComponentToComponent _returnvalue (Variables|Default|GetCapsuleComponent) "None" "KeepWorld" "KeepWorld" "KeepWorld" true)
  (Utilities|Array|Add (Variables|Default|GetHitboxes) _returnvalue)
  (Components|Sphere|SetSphereRadius (Variables|/Game/StylishCombatKit/Misc/BP_Hitbox.BP_Hitbox_C|GetHitbox _returnvalue) 7e+01 true)
  (Variables|/Game/StylishCombatKit/Misc/BP_Hitbox.BP_Hitbox_C|SetHitData _returnvalue (Utilities|Struct|MakeStruct_HitData 1 "0.000000,0.000000,1500.000000" 5e+01 2 0.0 0.2 3e+01))
  (Default|Activate _returnvalue true)
  (Pawn|Components|CharacterMovement|SetMovementMode (Variables|Character|GetCharacterMovement) "MOVE_Flying" 0)
  (bind _output_get (Variables|/Script/Engine.MovementComponent|SetVelocity (Variables|Character|GetCharacterMovement) (* (Transformation|GetActorForwardVector) (Variables|Default|GetSpeed))))
  (Variables|Default|SetPreviousFrameVelocity _output_get))

(fn ConstructionScript
  (|CallParentFunction))