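; BP_HealthShop is an interactable shop that sells health items to the player for money.
; On Interact, it casts the player to BP_BaseCharacter and checks that HealthLeft is below HealthItemMax and that Money covers the fixed price.
; A purchase adds one to HealthLeft, deducts the cost through ManageMoney and plays a sound at the Box component's relative location.
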(event EventInteract
  (params (Player :type Character%20Object%20Reference))
  (Utilities|IsValid Player
    (:Is%20Valid
      (bind _asbp_base_character (Utilities|Casting|CastToBP_BaseCharacter Player))
      (Variables|Default|SetPlayer _asbp_base_character)
      (if (< (Variables|/Game/StylishCombatKit/Main/BP_BaseCharacter.BP_BaseCharacter_C|GetHealthLeft _asbp_base_character) (Variables|/Game/StylishCombatKit/Main/BP_BaseCharacter.BP_BaseCharacter_C|GetHealthItemMax _asbp_base_character))
        (if (>= (Variables|/Game/StylishCombatKit/Main/BP_BaseCharacter.BP_BaseCharacter_C|GetMoney (Variables|Default|GetPlayer)) 200)
          (Variables|/Game/StylishCombatKit/Main/BP_BaseCharacter.BP_BaseCharacter_C|SetHealthLeft (Variables|Default|GetPlayer) (+ (Variables|/Game/StylishCombatKit/Main/BP_BaseCharacter.BP_BaseCharacter_C|GetHealthLeft (Variables|Default|GetPlayer)) 1))
          (Default|ManageMoney (Variables|Default|GetPlayer) -200)
          (Audio|PlaySoundatLocation "/Game/FFBLAZE/Sound/ShopOrCurrencySFX/purchased_sound.purchased_sound" (Variables|/Script/Engine.SceneComponent|GetRelativeLocation (Variables|Default|GetBox)) "0, 0, 0" 0.5 1.0 0.0 0 0 0))))))

(fn ConstructionScript)