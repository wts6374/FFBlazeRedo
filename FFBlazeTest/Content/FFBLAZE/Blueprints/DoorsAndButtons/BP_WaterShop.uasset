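; BP_WaterShop is an interactable shop that sells water item and soda refills to the player character.
; On Interact it casts the player to BP_BaseCharacter and checks that either stock is below its maximum and that Money covers the fixed price.
; It adds one to each stock not yet full, charges the same price either way through ManageMoney, and plays a purchase sound at the Box's relative location.
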(event EventInteract
  (params (Player :type Character%20Object%20Reference))
  (Utilities|IsValid Player
    (:Is%20Valid
      (bind _asbp_base_character (Utilities|Casting|CastToBP_BaseCharacter Player))
      (Variables|Default|SetPlayer _asbp_base_character)
      (if (or (< (Variables|/Game/StylishCombatKit/Main/BP_BaseCharacter.BP_BaseCharacter_C|GetWaterItemLeft _asbp_base_character) (Variables|/Game/StylishCombatKit/Main/BP_BaseCharacter.BP_BaseCharacter_C|GetWaterItemMax _asbp_base_character)) (< (Variables|/Game/StylishCombatKit/Main/BP_BaseCharacter.BP_BaseCharacter_C|GetSodaLeft _asbp_base_character) (Variables|/Game/StylishCombatKit/Main/BP_BaseCharacter.BP_BaseCharacter_C|GetSodaMax _asbp_base_character)))
        (if (>= (Variables|/Game/StylishCombatKit/Main/BP_BaseCharacter.BP_BaseCharacter_C|GetMoney (Variables|Default|GetPlayer)) 500)
          (if (< (Variables|/Game/StylishCombatKit/Main/BP_BaseCharacter.BP_BaseCharacter_C|GetWaterItemLeft (Variables|Default|GetPlayer)) (Variables|/Game/StylishCombatKit/Main/BP_BaseCharacter.BP_BaseCharacter_C|GetWaterItemMax (Variables|Default|GetPlayer)))
            (Variables|/Game/StylishCombatKit/Main/BP_BaseCharacter.BP_BaseCharacter_C|SetWaterItemLeft (Variables|Default|GetPlayer) (+ (Variables|/Game/StylishCombatKit/Main/BP_BaseCharacter.BP_BaseCharacter_C|GetWaterItemLeft (Variables|Default|GetPlayer)) 1)))
          (if (< (Variables|/Game/StylishCombatKit/Main/BP_BaseCharacter.BP_BaseCharacter_C|GetSodaLeft (Variables|Default|GetPlayer)) (Variables|/Game/StylishCombatKit/Main/BP_BaseCharacter.BP_BaseCharacter_C|GetSodaMax (Variables|Default|GetPlayer)))
            (Variables|/Game/StylishCombatKit/Main/BP_BaseCharacter.BP_BaseCharacter_C|SetSodaLeft (Variables|Default|GetPlayer) (+ (Variables|/Game/StylishCombatKit/Main/BP_BaseCharacter.BP_BaseCharacter_C|GetSodaLeft (Variables|Default|GetPlayer)) 1)))
          (Default|ManageMoney (Variables|Default|GetPlayer) -500)
          (Audio|PlaySoundatLocation "/Game/FFBLAZE/Sound/ShopOrCurrencySFX/purchased_sound.purchased_sound" (Variables|/Script/Engine.SceneComponent|GetRelativeLocation (Variables|Default|GetBox)) "0, 0, 0" 0.5 1.0 0.0 0 0 0))))))

(fn ConstructionScript)