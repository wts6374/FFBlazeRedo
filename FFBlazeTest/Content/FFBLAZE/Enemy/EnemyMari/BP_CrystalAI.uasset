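; BP_CrystalAI is an enemy character that locks onto the player, attacks with montages and drops MoneywaterRefill pickups on death.
; It simulates player input, turning the AI controller's action index into a camera-relative direction that picks each attack, followed by a timed button release.
; Tick drives the health widget, distance-based teleport taunts and anti-air reactions.
; Temperature tier swaps materials, gates attacks and sets TriggerActive.
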(event Custom|ChargeTimer
  ;[1 1 1] Attack command
  ;;[1 1 1] Input attack button and hold for specified charge time
  (bind _output_get (Variables|Default|SetLightButton false))
  (|CallParentFunction _output_get)
  (bind _output_get_2 (Variables|Default|SetHeavyButton false))
  (CallFunction|InputHeavyAttack _output_get_2))

(event Custom|ChangeLook
  (bind _mesh (Variables|Character|GetMesh))
  (bind _mesh_2 (Variables|Character|GetMesh))
  (bind _mesh_3 (Variables|Character|GetMesh))
  (bind _mesh_4 (Variables|Character|GetMesh))
  (bind _mesh_5 (Variables|Character|GetMesh))
  ;[1 1 1] Attack command
  ;;[1 1 1] Change material based on Temperature
  (switch int (Variables|Default|GetTempTier)
    (:0
      (Rendering|Material|SetMaterial _mesh_5 0 "/Game/FFBLAZE/Enemy/EnemyColors/Cool.Cool")
      (Rendering|Material|SetMaterial _mesh_5 1 "/Game/FFBLAZE/Enemy/EnemyColors/CoolOutline.CoolOutline"))
    (:1
      (Rendering|Material|SetMaterial _mesh_3 1 "/Game/FFBLAZE/Enemy/EnemyColors/WarmOutline.WarmOutline")
      (Rendering|Material|SetMaterial _mesh_3 0 "/Game/FFBLAZE/Enemy/EnemyColors/Warm.Warm"))
    (:2
      (Rendering|Material|SetMaterial _mesh_2 0 "/Game/FFBLAZE/Enemy/EnemyColors/Hottie.Hottie")
      (Rendering|Material|SetMaterial _mesh_2 1 "/Game/FFBLAZE/Enemy/EnemyColors/WarmOutline.WarmOutline"))
    (:3
      (Rendering|Material|SetMaterial _mesh 0 "/Game/FFBLAZE/Enemy/EnemyColors/RedHot.RedHot")
      (Rendering|Material|SetMaterial _mesh 1 "/Game/FFBLAZE/Enemy/EnemyColors/RedHotOutline.RedHotOutline"))
    (:4
      (Rendering|Material|SetMaterial _mesh_4 0 "/Game/FFBLAZE/Enemy/EnemyColors/WhiteHot.WhiteHot")
      (Rendering|Material|SetMaterial _mesh_4 1 "/Game/FFBLAZE/Enemy/EnemyColors/WhitHotOutline.WhitHotOutline"))))

(event Custom|UpdateUI
  (bind _healthwidget (Variables|Default|GetHealthWidget))
  ;[1 1 1] Update UI
  (Variables|/Game/FFBLAZE/UI/EnemyHealth.EnemyHealth_C|SetEnemy (Variables|Default|GetUIBar) self)
  (if (Variables|Default|GetIsLockedOn)
    (Rendering|SetVisibility _healthwidget true false)
    (else
      (Rendering|SetVisibility _healthwidget false false))))

(event Custom|StartUI
  ;[1 1 1] Update UI
  (bind _asenemy_health (Utilities|Casting|CastToEnemyHealth (UserInterface|GetUserWidgetObject (Variables|Default|GetHealthWidget))))
  (Variables|Default|SetUIBar _asenemy_health))

(event Custom|SpecialEvents
  (bind _charactermovement (Variables|Character|GetCharacterMovement))
  (bind _charactermovement_2 (Variables|Character|GetCharacterMovement))
  (bind _charactermovement_3 (Variables|Character|GetCharacterMovement))
  ;[1 1 1] Handle Teleports and anti-air events
  (if (Utilities|IsValid (Variables|Default|GetLockOnTarget))
    (if (and (>= (Math|Vector|Distance(Vector) (Transformation|GetActorLocation (Variables|Default|GetLockOnTarget)) (Transformation|GetActorLocation self)) 1.2e+03) (Variables|Default|GetCanAttack))
      (CallFunction|StartAnim)
      (CallFunction|CanDo false false)
      (CallFunction|RestoreMovementDefaults true)
      (CallFunction|OrientCharacter true false)
      (Variables|/Script/Engine.MovementComponent|SetVelocity _charactermovement_2 (+ (* (Transformation|GetActorForwardVector) 5e+01) "0, 0,100.000000"))
      (Variables|Default|SetFloatTime 0.2)
      (Variables|/Script/Engine.CharacterMovementComponent|SetGravityScale _charactermovement_2 2.0)
      (Variables|Default|SetStateIndex 1)
      (if (Variables|/Game/StylishCombatKit/Main/BP_BaseCharacter.BP_BaseCharacter_C|GetInAir (Variables|Default|GetLockOnTarget))
        (Animation|PlayAnimMontage "/Game/FFBLAZE/Enemy/EnemyWhip/E_TauntA.E_TauntA" 1.0 "")
        (Variables|Default|SetInputBuffer 0)
        (CallFunction|CanDo false true)
        (Effects|SpawnEmitteratLocation "/Game/StylishCombatKit/VFX/ParticleSystems/P_TeleportRed.P_TeleportRed" (Transformation|GetActorLocation))
        (Variables|/Script/Engine.CharacterMovementComponent|SetGravityScale _charactermovement 5.0)
        (Variables|/Script/Engine.MovementComponent|SetVelocity _charactermovement (+ (* (Variables|/Script/Engine.MovementComponent|GetVelocity _charactermovement) "0.700000,0.700000,0.000000") "0, 0,700.000000"))
        (Variables|Default|SetFloatTime 0.8)
        (Variables|Default|SetStateIndex 2)
        (Variables|Default|SetSubStateIndex 1)
        (else
          (Animation|PlayAnimMontage "/Game/FFBLAZE/Enemy/EnemyWhip/E_Taun.E_Taun" 1.0 "")
          (Variables|Default|SetInputBuffer 0)
          (CallFunction|CanDo false true)
          (Effects|SpawnEmitteratLocation "/Game/StylishCombatKit/VFX/ParticleSystems/P_TeleportRed.P_TeleportRed" (Transformation|GetActorLocation))))
      (elif (Math|Boolean|ANDBoolean (<= (Math|Vector|Distance(Vector) (Transformation|GetActorLocation (Variables|Default|GetLockOnTarget)) (Transformation|GetActorLocation self)) 25.0) (Variables|Default|GetCanAttack) (Variables|/Game/StylishCombatKit/Main/BP_BaseCharacter.BP_BaseCharacter_C|GetInAir (Variables|Default|GetLockOnTarget)))
        (CallFunction|StartAnim)
        (CallFunction|CanDo false false)
        (CallFunction|RestoreMovementDefaults true)
        (CallFunction|OrientCharacter true false)
        (Animation|PlayAnimMontage "/Game/FFBLAZE/Enemy/EnemyWhip/EAntiAir.EAntiAir" 1.0 "")
        (Variables|Default|SetStateIndex 2)
        (Variables|Default|SetSubStateIndex 1)
        (CallFunction|UpdateRecentMoves -1)
        (elif (and (== (Variables|Default|GetStateIndex) 2) (== (Variables|Default|GetSubStateIndex) 1))
          (CallFunction|StartAnim)
          (CallFunction|CanDo false false)
          (CallFunction|RestoreMovementDefaults true)
          (CallFunction|OrientCharacter true false)
          (Animation|PlayAnimMontage "/Game/FFBLAZE/Enemy/EnemyWhip/E_AttackRadius.E_AttackRadius" 1.0 "")
          (Variables|Default|SetStateIndex 2)
          (Variables|Default|SetSubStateIndex 5)
          (Variables|/Script/Engine.CharacterMovementComponent|SetGravityScale _charactermovement_3 5.0)
          (Variables|/Script/Engine.MovementComponent|SetVelocity _charactermovement_3 (+ (* (Variables|/Script/Engine.MovementComponent|GetVelocity _charactermovement_3) "0.700000,0.700000,0.000000") "0, 0,700.000000")))))))

(event EventBeginPlay
  ;[1 1 1] Initialize
  (|CallParentFunction)
  (bind _asbp_base_character (Utilities|Casting|CastToBP_BaseCharacter (Game|GetPlayerCharacter 0)))
  (Variables|Default|SetLockOnTarget _asbp_base_character)
  (Variables|Default|SetIsLockedOn true)
  (Variables|Default|SetLockonButton true)
  (CallFunction|StartUI))

(event EventCollisionStopTriggered
  ;[1 1 1] Dash Punch Collision Trigger
  (Animation|PlayAnimMontage "/Game/FFBLAZE/Enemy/EnemyWhip/E_DashKick.E_DashKick" 0.9 "ContactEnd"))

(event EventFlinch
  ;[1 1 1] Hurt animation
  (Animation|PlayAnimMontage (select (Variables|Default|GetInAir) "/Game/FFBLAZE/Enemy/EnemyWhip/E_HitAir.E_HitAir" "/Game/FFBLAZE/Enemy/EnemyWhip/E_Hit.E_Hit") 1.0 ""))

(event EventNeutralDirectionHoldButtonInput
  (bind _charactermovement (Variables|Character|GetCharacterMovement))
  ;[1 1 1] Dash Punch Collision Trigger
  (Animation|PlayAnimMontage "/Game/FFBLAZE/Enemy/EnemyWhip/E_AttackRadius.E_AttackRadius" 1.0 "")
  (Variables|Default|SetStateIndex 2)
  (Variables|Default|SetSubStateIndex 5)
  (Variables|Default|SetCollisionStop false)
  (Variables|Default|SetInputBuffer -1)
  (Variables|/Script/Engine.CharacterMovementComponent|SetGravityScale _charactermovement 5.0)
  (Variables|/Script/Engine.MovementComponent|SetVelocity (Variables|Character|GetCharacterMovement) (+ (* (Variables|/Script/Engine.MovementComponent|GetVelocity _charactermovement) "0.500000,0.500000,0.000000") "0, 0,600.000000"))
  (Variables|Default|SetFloatTime 0.2))

(event EventForceLand
  ;[1 1 1] Land
  (Variables|Default|SetInAir false)
  (if (and (== (Variables|Default|GetStateIndex) 2) (== (Variables|Default|GetSubStateIndex) 5))
    (Animation|PlayAnimMontage "/Game/FFBLAZE/Enemy/EnemyWhip/E_Combo.E_Combo" 1.0 "FinalHit")
    (CallFunction|ResetAirOptions :!label _label)
    (CallFunction|RestoreMovementDefaults false)
    (Variables|Default|SetCombatAnimation true)
    (Variables|Default|SetSubStateIndex 0)
    (elif (== (Variables|Default|GetStateIndex) 4)
      (Animation|PlayAnimMontage "/Game/FFBLAZE/Enemy/EnemyWhip/E_HitAir.E_HitAir" 1.0 "Land")
      (goto _label)
      (elif (== (Variables|Default|GetStateIndex) 5)
        (Animation|PlayAnimMontage "/Game/FFBLAZE/Enemy/EnemyWhip/E_Dead.E_Dead" 1.0 "Explode")
        (else
          (Animation|PlayAnimMontage "/Game/FFBLAZE/Enemy/EnemyWhip/E_Land.E_Land" 1.5 "Land")
          (CallFunction|CanDo true true)
          (CallFunction|ResetAirOptions)
          (CallFunction|StartAnim)
          (CallFunction|RestoreMovementDefaults false)
          (Variables|Default|SetCombatAnimation false)
          (CallFunction|ReleaseBuffer))))))

(event EventInputLightAttack
  (params (Pressed :type Boolean))
  (bind _rotation (CallFunction|CameraYaw))
  (bind _returnvalue (Transformation|GetActorLocation))
  (bind _aicontrollerref (Variables|Default|GetAIControllerRef))
  (bind _lockontarget (Variables|Default|GetLockOnTarget))
  (bind _returnvalue_2 (Transformation|GetActorLocation _lockontarget))
  (bind _aiactionindex (Variables|/Game/StylishCombatKit/AI/AIC_Enemy.AIC_Enemy_C|GetAIActionIndex _aicontrollerref))
  (bind _returnvalue_3 (Math|Vector|GetUnitDirection(Vector) _returnvalue _returnvalue_2))
  (bind (_x _y) (Math|Vector|BreakVector _returnvalue_3))
  (bind _returnvalue_4 (Math|Vector|MakeVector _x _y 0.0))
  (bind _returnvalue_5 (Math|Vector|Normalize _returnvalue_4))
  (bind _returnvalue_6 (Math|Vector|UnrotateVector _returnvalue_5 _rotation))
  (bind _returnvalue_7 (Math|Conversions|ToVector2D(Vector) _returnvalue_6))
  (bind (_x_2 _y_2) (Math|Vector2D|BreakVector2D _returnvalue_7))
  (bind _returnvalue_8 (Math|Vector2D|MakeVector2D _y_2 _x_2))
  (bind _returnvalue_9 (* _returnvalue_8 -1.0))
  ;[1 1 1] Attack command
  (if (and (Variables|Default|GetCanAttack) (> (Variables|Default|GetTempTier) 0))
    (if (not (Variables|Default|GetInAir))
      ;;[1 1 1] Set input vector to simulate directional inputs
      (Variables|Default|SetInputVector (Utilities|Select :Index _aiactionindex :Option%200 _returnvalue_9 :Option%201 "" :Option%202 _returnvalue_8 :Option%203 _returnvalue_9 :Option%204 "" :Option%205 _returnvalue_8))
      ;;[1 1 1] Input attack button and hold for specified charge time
      (if (>= _aiactionindex 3)
        (switch int (+ (select (== (Variables|Default|GetInputBuffer) 3) (Variables|Default|GetDirectionBuffer) (CallFunction|DirectionalInput)) 1)
          (:Default
            (Animation|PlayAnimMontage "/Game/FFBLAZE/Enemy/EnemyWhip/E_DashKick.E_DashKick" 1.0 "" :!label _label)
            (Variables|Default|SetStateIndex 2)
            (Variables|Default|SetSubStateIndex 7))
          (:0
            (Animation|PlayAnimMontage "/Game/FFBLAZE/Enemy/EnemyWhip/E_Whip.E_Whip" 1.0 "")
            (Variables|Default|SetStateIndex 2)
            (Variables|Default|SetSubStateIndex 8))
          (:1
            (goto _label))
          (:2
            (Animation|PlayAnimMontage "/Game/FFBLAZE/Enemy/EnemyWhip/E_AttackRadius.E_AttackRadius" 1.0 "")
            (Variables|Default|SetStateIndex 2)
            (Variables|Default|SetSubStateIndex 5)))
        (CallFunction|UpdateRecentMoves -1)
        (else
          (CallFunction|StartAnim)
          (CallFunction|CanDo false true)
          (CallFunction|OrientCharacter true true)
          (switch int (+ (select (== (Variables|Default|GetInputBuffer) 3) (Variables|Default|GetDirectionBuffer) (CallFunction|DirectionalInput)) 1)
            (:0
              (Animation|PlayAnimMontage "/Game/FFBLAZE/Enemy/EnemyWhip/EAntiAir.EAntiAir" 1.0 "")
              (Variables|Default|SetStateIndex 2)
              (Variables|Default|SetSubStateIndex 1))
            (:1
              (Animation|PlayAnimMontage "/Game/FFBLAZE/Enemy/EnemyWhip/E_Combo.E_Combo" 1.0 "")
              (Variables|Default|SetStateIndex 2)
              (Variables|Default|SetSubStateIndex 3))
            (:2
              (Animation|PlayAnimMontage "/Game/FFBLAZE/Enemy/EnemyWhip/E_Kick.E_Kick" 1.0 "")
              (Variables|Default|SetStateIndex 2)
              (Variables|Default|SetSubStateIndex 4)))
          (CallFunction|UpdateRecentMoves -1)))
      (Utilities|Time|SetTimerbyEvent (delegate Custom|ChargeTimer) 0.3))))

(event EventOnLanded
  (params (Hit :type Hit%20Result%20Structure%20%28by%20ref%29))
  ;[1 1 1] Land
  (Variables|Default|SetInAir false)
  (if (and (== (Variables|Default|GetStateIndex) 2) (== (Variables|Default|GetSubStateIndex) 5))
    (Animation|PlayAnimMontage "/Game/FFBLAZE/Enemy/EnemyWhip/E_Combo.E_Combo" 1.0 "FinalHit")
    (CallFunction|ResetAirOptions :!label _label)
    (CallFunction|RestoreMovementDefaults false)
    (Variables|Default|SetCombatAnimation true)
    (Variables|Default|SetSubStateIndex 0)
    (elif (== (Variables|Default|GetStateIndex) 4)
      (Animation|PlayAnimMontage "/Game/FFBLAZE/Enemy/EnemyWhip/E_HitAir.E_HitAir" 1.0 "Land")
      (goto _label)
      (elif (== (Variables|Default|GetStateIndex) 5)
        (Animation|PlayAnimMontage "/Game/FFBLAZE/Enemy/EnemyWhip/E_Dead.E_Dead" 1.0 "Explode")
        (else
          (Animation|PlayAnimMontage "/Game/FFBLAZE/Enemy/EnemyWhip/E_Land.E_Land" 1.5 "Land")
          (CallFunction|CanDo true true)
          (CallFunction|ResetAirOptions)
          (CallFunction|StartAnim)
          (CallFunction|RestoreMovementDefaults false)
          (Variables|Default|SetCombatAnimation false)
          (CallFunction|ReleaseBuffer))))))

(event EventHurtAnimation
  (params (AttackerHitbox :type BP%20Hitbox%20Object%20Reference))
  ;[1 1 1] Hurt animation
  (if (Variables|Default|GetInAir)
    (Animation|PlayAnimMontage "/Game/FFBLAZE/Enemy/EnemyWhip/E_HitAir.E_HitAir" 1.0 "")
    (Audio|PlaySound2D "/Game/FFBLAZE/Sound/EnemyHurtSFX/enemy_hurt1.enemy_hurt1" 0.2 1.0 0.0 0 0)
    (else
      (Animation|PlayAnimMontage "/Game/FFBLAZE/Enemy/EnemyWhip/E_Hit.E_Hit" 1.0 "")
      (Audio|PlaySound2D "/Game/FFBLAZE/Sound/EnemyHurtSFX/enemy_hurt2.enemy_hurt2" 0.2 1.0 0.0 0 0)))
  (CallFunction|StartAnim)
  (CallFunction|CanDo false true)
  (Variables|Default|SetCanEnemyStep false)
  (Variables|Default|SetStateIndex 4))

(event EventDeathAnimation
  ;[1 1 1] Hurt animation
  (Animation|PlayAnimMontage "/Game/FFBLAZE/Enemy/EnemyWhip/E_Dead.E_Dead" 1.0 "")
  (Audio|PlaySound2D "/Game/FFBLAZE/Sound/EnemyHurtSFX/enemy_die.enemy_die" 0.2 1.0 0.0 0 0)
  (Variables|Default|SetTargetGravity 0.0)
  (Variables|Default|SetFloatTime 3.0)
  (Utilities|FlowControl|Delay 1.3)
  (for _index (range 0 4)
    (Game|SpawnActorfromClass "/Game/FFBLAZE/Pickups/MoneywaterRefill.MoneywaterRefill_C" (Transformation|GetActorTransform) "Undefined" 0 0))
  (Actor|DestroyActor))

(event EventTick
  (params (DeltaSeconds :type Float%20%28single-precision%29))
  ;[1 1 1] Updater
  (|CallParentFunction DeltaSeconds)
  (CallFunction|ChangeLook)
  (CallFunction|UpdateUI)
  (CallFunction|SpecialEvents)
  (if (>= (Variables|Default|GetTempTier) 2)
    (Variables|Default|SetTriggerActive true)
    (else
      (Variables|Default|SetTriggerActive false))))

(fn ConstructionScript
  (bind _mesh (Variables|Character|GetMesh))
  (|CallParentFunction)
  (Transformation|AttachComponentToComponent (Variables|Default|GetHurtboxTorso) _mesh "spine_02" "KeepRelative" "KeepRelative" "KeepRelative" true)
  (Transformation|AttachComponentToComponent (Variables|Default|GetHurtboxLegL) _mesh "calf_l" "KeepRelative" "KeepRelative" "KeepRelative" true)
  (Transformation|AttachComponentToComponent (Variables|Default|GetHurtboxLegR) _mesh "calf_r" "KeepRelative" "KeepRelative" "KeepRelative" true)
  (Transformation|AttachComponentToComponent (Variables|Default|GetRepelSphere) _mesh "spine_02" "KeepRelative" "KeepRelative" "KeepRelative" true)
  (Variables|Default|SetHurtboxes (Utilities|Array|MakeArray (Variables|Default|GetHurtboxTorso) (Variables|Default|GetHurtboxLegL) (Variables|Default|GetHurtboxLegR))))