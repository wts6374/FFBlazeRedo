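; BP_CivilianDuplicate is an interactable civilian that the player rescues, likely as a collectible objective.
; The interact interface event fires through a DoOnce, disables the Box collision and plays a Rescue montage.
; After a delay it plays a coin sound, spawns a teleport particle at the civilian, and turns interaction off.
; Collected then hides the civilian, light and text render.
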(event Custom|Collected
  (Rendering|SetVisibility (Variables|Default|GetCivilian) false false)
  (Collision|SetCollisionEnabled (Variables|Default|GetBox) "NoCollision")
  (Rendering|SetVisibility (Variables|Default|GetPointLight) false false)
  (Rendering|SetVisibility (Variables|Default|GetTextRender) false false))

(event EventBeginPlay
  (Variables|Default|SetInteraction true))

(event EventTriggerInteractInterface
  (Utilities|FlowControl|DoOnce false
    (:Completed
      (Collision|SetCollisionEnabled (Variables|Default|GetBox) "NoCollision")
      (Animation|Montage|PlayMontage 0 "/Game/FFBLAZE/Pickups/Rescue.Rescue"
        (:then
          (Utilities|FlowControl|Delay 2.75)
          (Audio|PlaySoundatLocation "/Game/FFBLAZE/Sound/ShopOrCurrencySFX/collected_coin_sound.collected_coin_sound" "0,0.000000, 0" "0, 0, 0" 1.0 1.0 0.0 0 0 0)
          (Effects|SpawnEmitteratLocation "/Game/StylishCombatKit/VFX/ParticleSystems/P_TeleportBlue.P_TeleportBlue" (Transformation|GetActorLocation) "0, 0, 0" "1.000000,1.000000,1.000000" false)
          (Rendering|SetVisibility (Variables|Default|GetCivilian) false false)
          (Collision|SetCollisionEnabled (Variables|Default|GetBox) "NoCollision")
          (Variables|Default|SetInteraction false)
          (CallFunction|Collected))))))

(fn ConstructionScript)