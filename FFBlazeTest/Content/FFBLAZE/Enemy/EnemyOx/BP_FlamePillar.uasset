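; Flame pillar attack for the Ox enemy, built on a parent class that supplies initialization, hit tracking and orientation helpers.
; On Initialize it plays the Spew animation and montage, appearing at the owner's lock-on target with a fixed rotation and soft-lock orientation, or otherwise at the owner's location.
; Each tick it runs the hit-reset check and counts Duration down by custom time dilation, destroying itself at zero.
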(event EventBeginPlay
  (|CallParentFunction) ; This node is disabled and will not be called.\nDrag off pins to build functionality.
)

(event EventTick
  (params (DeltaSeconds :type Float%20%28single-precision%29))
  ;[1 1 1] Update values on tick
  (|CallParentFunction DeltaSeconds)
  (CallFunction|ResetHitsCheck)
  (if (> (Variables|Default|GetDuration) 0.0)
    (Variables|Default|SetDuration (Math|Float|Clamp(Float) (- (Variables|Default|GetDuration) (* DeltaSeconds (Variables|Default|GetCustomTimeDilation))) 0.0 (Variables|Default|GetDuration))))
  (if (== (Variables|Default|GetDuration) 0.0)
    (CallFunction|Destroy)))

(event EventInitialize
  (bind _ownercharacter (Variables|Default|GetOwnerCharacter))
  (bind _ownercharacter_2 (Variables|Default|GetOwnerCharacter))
  (bind _mesh (Variables|Character|GetMesh))
  ;[1 1 1] Initialize
  (|CallParentFunction)
  (Rendering|SetVisibility _mesh true false)
  (Audio|Components|Audio|Stop _mesh)
  (Components|Animation|PlayAnimation _mesh "/Game/FFBLAZE/Enemy/EnemyOx/Spew.Spew" false)
  (Rendering|SetVisibility _mesh true false)
  (CallFunction|StartAnim)
  (if (and (Variables|/Game/StylishCombatKit/Main/BP_BaseCharacter.BP_BaseCharacter_C|GetIsLockedOn _ownercharacter_2) (Utilities|IsValid (Variables|/Game/StylishCombatKit/Main/BP_BaseCharacter.BP_BaseCharacter_C|GetLockOnTarget _ownercharacter_2)))
    (Transformation|SetActorLocation (Transformation|GetActorLocation (Variables|/Game/StylishCombatKit/Main/BP_BaseCharacter.BP_BaseCharacter_C|GetLockOnTarget _ownercharacter)) false false)
    (Transformation|SetActorRotation "0,90.000000, 0")
    (CallFunction|OrientCharacter false true)
    (else
      (Transformation|SetActorTransform (Math|Conversions|ToTransform(Vector) (Transformation|GetActorLocation _ownercharacter)))))
  (Animation|PlayAnimMontage "/Game/FFBLAZE/Enemy/EnemyOx/Spew.Spew" 1.1 "None"))

(fn ConstructionScript
  (|CallParentFunction))