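; BP_XrossSlash is a slash projectile in StylishCombatKit that carries a damaging hitbox with an upward launch.
; On Initialize it runs the parent logic, then spawns a spherical BP_Hitbox, attaches it to its capsule slightly forward, fills its hit data and activates it.
; If the owner is locked onto a valid target, it redirects velocity along the owner-to-target line at unchanged speed and adjusts only its pitch to match.
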(event EventBeginPlay
  (|CallParentFunction) ; This node is disabled and will not be called.\nDrag off pins to build functionality.
)

(event Collision|EventActorBeginOverlap
  (params (OtherActor :type Actor%20Object%20Reference)))

(event EventTick
  (params (DeltaSeconds :type Float%20%28single-precision%29))
  (|CallParentFunction DeltaSeconds) ; This node is disabled and will not be called.\nDrag off pins to build functionality.
)

(event EventInitialize
  (bind _returnvalue (Transformation|GetActorRotation))
  (bind _charactermovement (Variables|Character|GetCharacterMovement))
  (bind (_roll _pitch _yaw) (Math|Rotator|BreakRotator _returnvalue))
  ;[1 1 1] Initialize
  (|CallParentFunction)
  (bind _returnvalue_2 (Game|SpawnActorfromClass "/Game/StylishCombatKit/Misc/BP_Hitbox.BP_Hitbox_C" (Transformation|GetActorTransform) "AlwaysSpawn" 0 0))
  (Variables|/Game/StylishCombatKit/Misc/BP_Hitbox.BP_Hitbox_C|SetOwnerCharacter _returnvalue_2 self)
  (Transformation|AttachComponentToComponent _returnvalue_2 (Variables|Default|GetCapsuleComponent) "None" "KeepWorld" "KeepWorld" "KeepWorld" true)
  (Utilities|Array|Add (Variables|Default|GetHitboxes) _returnvalue_2)
  (Variables|/Game/StylishCombatKit/Misc/BP_Hitbox.BP_Hitbox_C|SetHitData _returnvalue_2 (Utilities|Struct|MakeStruct_HitData 0 "0.000000,0.000000,200.000000" 4.0 2 0.01 0.02 3.0 true 25.0))
  (Components|Sphere|SetSphereRadius (Variables|/Game/StylishCombatKit/Misc/BP_Hitbox.BP_Hitbox_C|GetHitbox _returnvalue_2) 9e+01 true)
  (Transformation|SetActorRelativeLocation _returnvalue_2 "100.000000, 0, 0")
  (Default|Activate _returnvalue_2 true)
  (if (and (Variables|/Game/StylishCombatKit/Main/BP_BaseCharacter.BP_BaseCharacter_C|GetIsLockedOn (Variables|Default|GetOwnerCharacter)) (Utilities|IsValid (Variables|/Game/StylishCombatKit/Main/BP_BaseCharacter.BP_BaseCharacter_C|GetLockOnTarget (Variables|Default|GetOwnerCharacter))))
    (bind _output_get (Variables|/Script/Engine.MovementComponent|SetVelocity _charactermovement (* (Math|Vector|GetUnitDirection(Vector) (Transformation|GetActorLocation (Variables|Default|GetOwnerCharacter)) (Transformation|GetActorLocation (Variables|/Game/StylishCombatKit/Main/BP_BaseCharacter.BP_BaseCharacter_C|GetLockOnTarget (Variables|Default|GetOwnerCharacter)))) (Math|Vector|VectorLength (Variables|/Script/Engine.MovementComponent|GetVelocity _charactermovement)))))
    (Variables|Default|SetPreviousFrameVelocity _output_get)
    (Transformation|SetActorRotation (Math|Rotator|MakeRotator _roll (.Pitch (Math|Rotator|BreakRotator (Math|Rotator|FindLookatRotation (Transformation|GetActorLocation (Variables|Default|GetOwnerCharacter)) (Transformation|GetActorLocation (Variables|/Game/StylishCombatKit/Main/BP_BaseCharacter.BP_BaseCharacter_C|GetLockOnTarget (Variables|Default|GetOwnerCharacter)))))) _yaw))))

(fn ConstructionScript
  (|CallParentFunction))