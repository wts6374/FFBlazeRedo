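; BP_IceMove is a Stylish Combat Kit ice attack projectile that flies straight down, dealing damage with water and cooling effects.
; On Initialize it spawns a sphere BP_Hitbox attached to its capsule, fills in the hit data and activates it.
; Its CharacterMovement component drives the descent in Flying mode.
; Tick runs the reset-hits check and counts down Duration by custom time dilation, destroying the actor at zero.
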(event EventBeginPlay
  (|CallParentFunction) ; This node is disabled and will not be called.\nDrag off pins to build functionality.
)

(event Collision|EventActorBeginOverlap
  (params (OtherActor :type Actor%20Object%20Reference)))

(event EventTick
  (params (DeltaSeconds :type Float%20%28single-precision%29))
  ;[1 1 1] Update values on tick
  (|CallParentFunction DeltaSeconds)
  (CallFunction|ResetHitsCheck)
  (if (> (Variables|Default|GetDuration) 0.0)
    (Variables|Default|SetDuration (Math|Float|Clamp(Float) (- (Variables|Default|GetDuration) (* DeltaSeconds (Variables|Default|GetCustomTimeDilation))) 0.0 (Variables|Default|GetDuration))))
  (if (== (Variables|Default|GetDuration) 0.0)
    (CallFunction|Destroy)))

(event EventInitialize
  ;[1 1 1] Initialize
  (|CallParentFunction)
  (bind _returnvalue (Game|SpawnActorfromClass "/Game/StylishCombatKit/Misc/BP_Hitbox.BP_Hitbox_C" (Transformation|GetActorTransform) "AlwaysSpawn" 0 0))
  (Variables|/Game/StylishCombatKit/Misc/BP_Hitbox.BP_Hitbox_C|SetOwnerCharacter _returnvalue self)
  (Transformation|AttachComponentToComponent _returnvalue (Variables|Default|GetCapsuleComponent) "None" "KeepWorld" "KeepWorld" "KeepWorld" true)
  (Utilities|Array|Add (Variables|Default|GetHitboxes) _returnvalue)
  (Components|Sphere|SetSphereRadius (Variables|/Game/StylishCombatKit/Misc/BP_Hitbox.BP_Hitbox_C|GetHitbox _returnvalue) 8e+01 true)
  (Variables|/Game/StylishCombatKit/Misc/BP_Hitbox.BP_Hitbox_C|SetHitData _returnvalue (Utilities|Struct|MakeStruct_HitData 0 "0.000000,0.000000,-100.000000" 16.0 2 0.3 0.01 0.0 true 5e+01))
  (Default|Activate _returnvalue true)
  (Pawn|Components|CharacterMovement|SetMovementMode (Variables|Character|GetCharacterMovement) "MOVE_Flying" 0)
  (bind _output_get (Variables|/Script/Engine.MovementComponent|SetVelocity (Variables|Character|GetCharacterMovement) "0, 0,-2000.000000"))
  (Variables|Default|SetPreviousFrameVelocity _output_get))

(fn ConstructionScript
  (|CallParentFunction))